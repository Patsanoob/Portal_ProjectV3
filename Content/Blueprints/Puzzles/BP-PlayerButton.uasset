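; Puzzle button that, once pressed, marks its attached spline paths valid and turns its pad's grid green.
; On BeginPlay it finds attached BPSpline actors by endpoint proximity and creates the pad's dynamic material.
; PressButton ignores presses while down or moving, otherwise a timeline lowers the button.
; With Timer set, a retriggerable delay reverses the timeline, invalidating the paths and turning the grid white.
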(event Custom|Button%20Pressed
  ;[1 1 1] Button Movement
  (bind (_direction _alpha) (Timeline|TL-ButtonPressed Play)
    (:Update
      (Transformation|SetRelativeLocation (Variables|Default|GetSM-Button) (Math|Vector|Lerp(Vector) "0, 0, 0" "0, 0,-2.000000" _alpha) false false))
    (:Finished
      (switch Utilities|FlowControl|Switch|SwitchonETimelineDirection _direction
        (:Forward
          (Variables|Default|SetButton%20Down true)
          (CallFunction|PuzzleComplete)
          (if (Variables|Default|GetTimer)
            (Utilities|FlowControl|RetriggerableDelay (Variables|Default|GetDuration%20Reset))
            (CallFunction|ButtonDeactivate)))
        (:Backward
          (Variables|Default|SetButton%20Down false)
          (CallFunction|PuzzleIncomplete))))))

(event Custom|Button%20Deactivate
  ;[1 1 1] Button Movement
  (bind (_direction _alpha) (Timeline|TL-ButtonPressed Reverse)
    (:Update
      (Transformation|SetRelativeLocation (Variables|Default|GetSM-Button) (Math|Vector|Lerp(Vector) "0, 0, 0" "0, 0,-2.000000" _alpha) false false))
    (:Finished
      (switch Utilities|FlowControl|Switch|SwitchonETimelineDirection _direction
        (:Forward
          (Variables|Default|SetButton%20Down true)
          (CallFunction|PuzzleComplete)
          (if (Variables|Default|GetTimer)
            (Utilities|FlowControl|RetriggerableDelay (Variables|Default|GetDuration%20Reset))
            (CallFunction|ButtonDeactivate)))
        (:Backward
          (Variables|Default|SetButton%20Down false)
          (CallFunction|PuzzleIncomplete))))))

(event EventBeginPlay
  (Components|Timeline|SetPlayRate (Variables|Default|GetTL-ButtonPressed) 2.0)
  (CallFunction|GetLinesAttached)
  (bind _returnvalue (Rendering|Material|CreateDynamicMaterialInstance (Variables|Default|GetSM-Pad) 0 (Rendering|Material|GetMaterial (Variables|Default|GetSM-Pad) 0) "None" :!class /Script/Engine.PrimitiveComponent))
  (Variables|Default|SetMaterial _returnvalue)
  (Rendering|Material|SetVectorParameterValue (Variables|Default|GetMaterial) "GridColor" "(R=1.000000,G=1.000000,B=1.000000,A=1.000000)" :!class /Script/Engine.MaterialInstanceDynamic)
  (Rendering|Material|SetMaterial (Variables|Default|GetSM-Pad) 0 (Variables|Default|GetMaterial)))

(fn ConstructionScript)

(fn PuzzleComplete
  (for _array_element (Variables|Default|GetSpline%20Connected)
    (Default|PathValid _array_element true))
  (Rendering|Material|SetVectorParameterValue (Variables|Default|GetMaterial) "GridColor" "(R=0.000000,G=1.000000,B=0.000000,A=1.000000)" :!class /Script/Engine.MaterialInstanceDynamic))

(fn GetLinesAttached
  (bind _outactors (Actor|GetAllActorsOfClass "/Game/Blueprints/Puzzles/BP-Spline.BP-Spline_C"))
  (for _array_element _outactors
    (if (or (< (Math|Vector|Distance(Vector) (Transformation|GetActorLocation) (.Start (Default|GetFirstandLastPoint _array_element))) 6e+01) (< (Math|Vector|Distance(Vector) (.End (Default|GetFirstandLastPoint _array_element)) (Transformation|GetActorLocation)) 6e+01))
      (Utilities|Array|AddUnique (Variables|Default|GetSpline%20Connected) _array_element))))

(fn PressButton
  (if (not (or (Variables|Default|GetButton%20Down) (Audio|Components|Audio|IsPlaying (Variables|Default|GetTL-ButtonPressed))))
    (CallFunction|ButtonPressed)))

(fn PuzzleIncomplete
  (for _array_element (Variables|Default|GetSpline%20Connected)
    (Default|PathValid _array_element false))
  (Rendering|Material|SetVectorParameterValue (Variables|Default|GetMaterial) "GridColor" "(R=1.000000,G=1.000000,B=1.000000,A=1.000000)" :!class /Script/Engine.MaterialInstanceDynamic))