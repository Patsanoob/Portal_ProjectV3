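; Puzzle cable indicator that paints a spline path onto surfaces with decals and shows whether the connection is valid.
; The construction script box-traces the surface near the spline's end to orient the final icon decal.
; CreateTheDecals, run on BeginPlay and ShowPath, traces each inner segment and spaces surface-aligned decals along it with dynamic materials.
; PathValid tints them green or red, swaps the icon's locked/unlocked material and calls CallChangedState.
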(event Custom|Show%20Path
  (CallFunction|CreatetheDecals))

(event EventBeginPlay
  (CallFunction|CreatetheDecals)
  (CallFunction|PathValid false))

(fn ConstructionScript
  (bind _spline (Variables|Default|GetSpline))
  (bind _spline_2 (Variables|Default|GetSpline))
  (bind _spline_3 (Variables|Default|GetSpline))
  (bind _returnvalue (Spline|GetNumberOfSplinePoints _spline_3))
  (bind _returnvalue_2 (Spline|GetNumberOfSplinePoints _spline))
  (bind _returnvalue_3 (- _returnvalue_2 2))
  (bind _returnvalue_4 (- _returnvalue 3))
  (bind _returnvalue_5 (Spline|GetTransformatSplinePoint _spline_2 _returnvalue_3 "World" false))
  (bind (_start _end) (CallFunction|GetVectorPoints _returnvalue_4 "World"))
  (Utilities|FlowControl|Sequence
    (:then_0
      ;[1 1 1] Setup the Final Icon for the Spline
      (bind (_outhit _returnvalue_6) (Class|KismetSystemLibrary|BoxTraceSingleforObjects (.location _returnvalue_5) (+ (.location _returnvalue_5) "0.100000,0.000000,0") "1.000000,1.000000,1.000000" "0, 0, 0" (Utilities|Array|MakeArray "ObjectTypeQuery8" "ObjectTypeQuery9") false 0 "None" true))
      (if _returnvalue_6
        (LocalVariables|SetL-UpVect (.Normal (Collision|BreakHitResult _outhit)))
        (LocalVariables|SetL-Transform (Transformation|GetWorldTransform (.HitComponent (Collision|BreakHitResult _outhit))))
        (Transformation|SetRelativeLocation (Variables|Default|GetDecal) (|GetLastLocation) false false)
        (LocalVariables|SetL-Relative%20Location%201 (Math|Transform|InverseTransformLocation (LocalVariables|GetL-Transform) _start))
        (LocalVariables|SetL-Relative%20Location%202 (Math|Transform|InverseTransformLocation (LocalVariables|GetL-Transform) _end))
        (LocalVariables|SetL-Relative%20Decal%20Location (Math|Transform|InverseTransformLocation (LocalVariables|GetL-Transform) (Transformation|GetWorldLocation (Variables|Default|GetDecal))))
        (Transformation|SetWorldRotation (Variables|Default|GetDecal) (Math|Rotator|MakeRotator (Math|Float|SelectFloat 9e+01 (- (Math|Float|Absolute(Float) (.yaw (Math|Rotator|MakeRotfromX (Math|Vector|Normalize (- (LocalVariables|GetL-Relative%20Location%201) (LocalVariables|GetL-Relative%20Location%202)))))) (Math|Float|SelectFloat -9e+01 9e+01 (Math|Float|NearlyEqual(Float) (.Z (Math|Vector|BreakVector (LocalVariables|GetL-UpVect))) 1.0 1e-06))) (Math|Float|NearlyEqual(Float) (.Z (Math|Vector|BreakVector (LocalVariables|GetL-UpVect))) 0.0 1e-06)) (.Pitch (Math|Rotator|BreakRotator (Math|Rotator|MakeRotfromX (LocalVariables|GetL-UpVect)))) (.Yaw (Math|Rotator|BreakRotator (Math|Rotator|MakeRotfromX (LocalVariables|GetL-UpVect))))) false false)))))

(fn PathValid
  (params (Valid :type Boolean))
  (Variables|Default|SetValid%20Cable Valid)
  (for _array_element (Variables|Default|GetMaterial)
    (Rendering|Material|SetVectorParameterValue _array_element "Color" (Math|Color|SelectColor "(R=0.000000,G=0.501961,B=0.000000,A=1.000000)" "(R=1.000000,G=0.000000,B=0.000000,A=1.000000)" (Variables|Default|GetValid%20Cable)) :!class /Script/Engine.MaterialInstanceDynamic))
  (Rendering|Components|Decal|SetDecalMaterial (Variables|Default|GetDecal) (select (Variables|Default|GetValid%20Cable) "/Game/Assets/Material/Decals/MD-UnLocked.MD-UnLocked" "/Game/Assets/Material/Decals/MD-Locked.MD-Locked"))
  (Default|CallChangedState))

(fn GetFirstandLastPoint
  (return (Spline|GetLocationatSplinePoint (Variables|Default|GetSpline) 0 "World") (Spline|GetLocationatSplinePoint (Variables|Default|GetSpline) (Spline|GetNumberOfSplinePoints (Variables|Default|GetSpline)) "World")))

(fn GetSplinePointLocation
  (params (Index :type Integer) (CoordinateSpace :type ESplineCoordinateSpace%20Enum :default "Local"))
  (return (.location (Spline|GetTransformatSplinePoint (Variables|Default|GetSpline) Index CoordinateSpace false))))

(fn GetVectorPoints
  (params (Index :type Integer) (CoordinateSpace :type ESplineCoordinateSpace%20Enum :default "World"))
  (LocalVariables|SetL-ExtraOffset (* (Math|Vector|Normalize (- (CallFunction|GetSplinePointLocation Index CoordinateSpace) (CallFunction|GetSplinePointLocation (+ Index 1) CoordinateSpace))) ""))
  (LocalVariables|SetL-Start (+ (CallFunction|GetSplinePointLocation Index CoordinateSpace) (LocalVariables|GetL-ExtraOffset)))
  (LocalVariables|SetL-End (- (CallFunction|GetSplinePointLocation (+ Index 1) CoordinateSpace) (LocalVariables|GetL-ExtraOffset)))
  (return (LocalVariables|GetL-Start) (LocalVariables|GetL-End)))

(fn IsPointonCorner
  (params (Index :type Integer))
  (bind _return_location (CallFunction|GetSplinePointLocation Index "World"))
  (bind _outhits (Class|KismetSystemLibrary|BoxTraceMultiforObjects _return_location (+ _return_location "0.100000,0.100000,0.100000") "5.000000,5.000000,5.000000" "0, 0, 0" (Utilities|Array|MakeArray "ObjectTypeQuery8" "ObjectTypeQuery9") false 0 "None" true))
  (return (> (Utilities|Array|Length _outhits) 1)))

(fn CreatetheDecals
  (for _array_element (Variables|Default|GetDecal%20List)
    (Utilities|IsValid _array_element
      (:Is%20Valid
        (Components|DestroyComponent _array_element))))
  (Utilities|Array|Clear (Variables|Default|GetMaterial))
  (for _index (range 1 (- (Spline|GetNumberOfSplinePoints (Variables|Default|GetSpline)) 3))
    (LocalVariables|SetL-Index _index)
    (LocalVariables|SetL-Direction (Math|Vector|Normalize (- (.End (CallFunction|GetVectorPoints (LocalVariables|GetL-Index) "World")) (.Start (CallFunction|GetVectorPoints (LocalVariables|GetL-Index) "World")))))
    (bind _output_get (LocalVariables|SetL-SpawnLocation (/ (+ (.Start (CallFunction|GetVectorPoints (LocalVariables|GetL-Index) "World")) (.End (CallFunction|GetVectorPoints (LocalVariables|GetL-Index) "World"))) 2.0)))
    (bind (_outhit _returnvalue) (Class|KismetSystemLibrary|BoxTraceSingleforObjects _output_get (+ _output_get "0.100000,0.100000,0.100000") "5.000000,5.000000,5.000000" "0, 0, 0" (Utilities|Array|MakeArray "ObjectTypeQuery8" "ObjectTypeQuery9") false 0 "ForDuration" true))
    (if _returnvalue
      (LocalVariables|SetL-Normal (.Normal (Collision|BreakHitResult _outhit)))
      (for _index_2 (range 0 (Math|Float|Truncate (|GetScale+TilingSize (LocalVariables|GetL-Index))))
        (bind _output_get_2 (LocalVariables|SetL-IndexIndent _index_2))
        (bind _returnvalue_2 (AddComponent|AddDecalComponent false (Math|Transform|MakeTransform (+ (* _output_get_2 (LocalVariables|GetL-Direction) 20) (.Start (CallFunction|GetVectorPoints (LocalVariables|GetL-Index) "Local"))) (Math|Rotator|MakeRotfromX (LocalVariables|GetL-Normal)) "1.000000,1.000000,1.000000")))
        (bind _output_get_3 (LocalVariables|SetL-DecalRef _returnvalue_2))
        (Utilities|Array|Add (Variables|Default|GetDecal%20List) _output_get_3)
        (bind _returnvalue_3 (Rendering|Material|CreateDynamicMaterialInstance "/Game/Assets/Material/Decals/MI_Decal-Light.MI_Decal-Light" "M-Decal" "None" :!class /Script/Engine.KismetMaterialLibrary))
        (Utilities|Array|Add (Variables|Default|GetMaterial) _returnvalue_3)
        (Rendering|Material|SetScalarParameterValue _returnvalue_3 "U Tiling" 1.0 :!class /Script/Engine.MaterialInstanceDynamic)
        (Rendering|Components|Decal|SetDecalMaterial (LocalVariables|GetL-DecalRef) _returnvalue_3)))))