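; Puzzle energy projectile that bounces around until it reaches a receiver, completing the puzzle and shutting down its spawner.
; Hit reactions use a cast chain: spawners and barriers destroy it, the first-person character dies, and other surfaces spark.
; Barrier overlaps, too many bounces, or a retriggerable, self-repeating timer finding it too far from its spawner also destroy it.
; Every failed end asks the spawner for a replacement.
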(event OnComponentBeginOverlap(CollisionComponent)
  (params (OverlappedComponent :type Primitive%20Component%20Object%20Reference) (OtherActor :type Actor%20Object%20Reference) (OtherComp :type Primitive%20Component%20Object%20Reference) (OtherBodyIndex :type Integer) (bFromSweep :type Boolean) (SweepResult :type Hit%20Result%20Structure%20%28by%20ref%29))
  (Utilities|Casting|CastToBP-Barrier OtherActor)
  (Default|SpawnEnergy (Variables|Default|GetSpawnerRef) 3.0)
  (Actor|DestroyActor))

(event Custom|Delay%20Death
  (Utilities|FlowControl|RetriggerableDelay 15.0)
  (if (> (Transformation|GetDistanceTo (Variables|Default|GetSpawnerRef) self) 4e+03)
    (Default|SpawnEnergy (Variables|Default|GetSpawnerRef) 3.0)
    (Actor|DestroyActor)
    (else
      (CallFunction|DelayDeath))))

(event Collision|EventHit
  (params (MyComp :type Primitive%20Component%20Object%20Reference) (Other :type Actor%20Object%20Reference) (OtherComp :type Primitive%20Component%20Object%20Reference) (bSelfMoved :type Boolean) (HitLocation :type Vector :default "0, 0, 0") (HitNormal :type Vector :default "0, 0, 0") (NormalImpulse :type Vector :default "0, 0, 0") (Hit :type Hit%20Result%20Structure%20%28by%20ref%29))
  (Math|Integer|IncrementInt (Variables|Default|GetBounce%20Count)
    (:%20%20
      (CallFunction|ManageCollisions Other HitLocation HitNormal))))

(fn ConstructionScript)

(fn ManageCollisions
  (params (Actor%20Hit :type Actor%20Object%20Reference) (Hit%20Location :type Vector) (Hit%20Normal :type Vector))
  (Utilities|FlowControl|Sequence
    (:then_0
      (Utilities|Casting|CastToBP-ProjectileSpawner Actor%20Hit
        (:then
          (Default|SpawnEnergy (Variables|Default|GetSpawnerRef) 3.0)
          (Actor|DestroyActor))
        (:CastFailed
          (bind _asbp_projectile_receiver (Utilities|Casting|CastToBP-ProjectileReceiver Actor%20Hit)
            (:then
              (Default|PuzzleComplete _asbp_projectile_receiver)
              (Default|ShutdownSpawner (Variables|Default|GetSpawnerRef))
              (Actor|DestroyActor))
            (:CastFailed
              (Utilities|Casting|CastToBP-Barrier Actor%20Hit
                (:then
                  (Default|SpawnEnergy (Variables|Default|GetSpawnerRef) 3.0)
                  (Actor|DestroyActor))
                (:CastFailed
                  (bind _asbp_first_person_character (Utilities|Casting|CastToBP_FirstPersonCharacter Actor%20Hit)
                    (:then
                      (Default|Death _asbp_first_person_character))
                    (:CastFailed
                      (Niagara|SpawnSystematLocation "/Game/Assets/Particle/NS-Spark.NS-Spark" Hit%20Location (Math|Rotator|MakeRotfromX Hit%20Normal)))))))))))
    (:then_1
      (if (> (Variables|Default|GetBounce%20Count) 5)
        (Default|SpawnEnergy (Variables|Default|GetSpawnerRef) 3.0)
        (Actor|DestroyActor)
        (else
          (CallFunction|DelayDeath))))))