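; Companion cube for portal puzzles: a physics prop carried by physics handles, with support for portal clones.
; Pickup and drop toggle gravity and material, while tick clamps velocity magnitude.
; Collision swaps between block and overlap on the cube and portal wall, and clone cubes attach to a clone's rifle handle.
; Touching a barrier's box releases the cube, plays a despawn effect, hides it and has its spawner create another.
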(event OnComponentBeginOverlap(StaticMesh)
  (params (OverlappedComponent :type Primitive%20Component%20Object%20Reference) (OtherActor :type Actor%20Object%20Reference) (OtherComp :type Primitive%20Component%20Object%20Reference) (OtherBodyIndex :type Integer) (bFromSweep :type Boolean) (SweepResult :type Hit%20Result%20Structure%20%28by%20ref%29))
  (bind _physicshandleref (Variables|Default|GetPhysicsHandleRef))
  (bind _asbp_barrier (Utilities|Casting|CastToBP-Barrier OtherActor))
  (if (== (Variables|/Game/Blueprints/LevelDesign/BP-Barrier.BP-Barrier_C|GetBox _asbp_barrier) OtherComp)
    (Utilities|IsValid _physicshandleref
      (:Is%20Valid
        (Physics|Components|PhysicsHandle|ReleaseComponent _physicshandleref)
        (CallFunction|CubeDestroyed))
      (:Is%20Not%20Valid
        (CallFunction|CubeDestroyed)))))

(event OnComponentHit(StaticMesh)
  (params (HitComponent :type Primitive%20Component%20Object%20Reference) (OtherActor :type Actor%20Object%20Reference) (OtherComp :type Primitive%20Component%20Object%20Reference) (NormalImpulse :type Vector :default "0, 0, 0") (Hit :type Hit%20Result%20Structure%20%28by%20ref%29)))

(event Custom|Cube%20Destroyed
  (Physics|SetSimulatePhysics (Variables|Default|GetStaticMesh) true)
  (Niagara|SpawnSystemAttached "/Game/Assets/Particle/NS_CubeDespawn.NS_CubeDespawn" (Variables|Default|GetStaticMesh) "None" "0, 0, 0" "0, 0, 0" "KeepRelativeOffset" false)
  (Utilities|FlowControl|Delay 1.0)
  (Development|SetHiddeninGame (Variables|Default|GetStaticMesh) true false)
  (Utilities|FlowControl|Delay 2.5)
  (Default|SpawnCube (Variables|Default|GetSpawner)))

(event EventTick
  (params (DeltaSeconds :type Float%20%28single-precision%29))
  (Physics|SetPhysicsLinearVelocity (Variables|Default|GetStaticMesh) (Math|Vector|ClampVectorSize (Transformation|GetVelocity) 0.0 (Variables|Default|GetClamp%20Velocity%20Z)) false "None"))

(event EventBeginPlay
  (if (Utilities|Operators|EqualEqual :A (Variables|Default|GetSpawn%20Loc))
    (Variables|Default|SetSpawn%20Loc (Transformation|GetActorLocation))
    (Variables|Default|SetSpawn%20Rot (Transformation|GetActorRotation))
    (bind _aspc_portal (Utilities|Casting|CastToPC-Portal (Game|GetPlayerController 0)))
    (Variables|Default|SetAs%20PC-Portal _aspc_portal)))

(fn ConstructionScript)

(fn Swap-Collision
  (params (Normal%20Collision :type Boolean) (Portal%20Ref :type B-Portal%20Object%20Reference))
  (if Normal%20Collision
    (Collision|SetCollisionResponsetoChannel (Variables|Default|GetStaticMesh) "ECC_GameTraceChannel4" "ECR_Block")
    (Utilities|IsValid Portal%20Ref
      (:Is%20Valid
        (Default|UpdateWallCollisionCube Portal%20Ref "ECC_WorldStatic" "ECC_GameTraceChannel11" "ECR_Block")))
    (else
      (Collision|SetCollisionResponsetoChannel (Variables|Default|GetStaticMesh) "ECC_GameTraceChannel4" "ECR_Overlap")
      (Utilities|IsValid Portal%20Ref
        (:Is%20Valid
          (Default|UpdateWallCollisionCube Portal%20Ref "ECC_WorldStatic" "ECC_GameTraceChannel11" "ECR_Overlap"))))))

(fn CubePickedUp
  (params (PhysicsHandle%20Picking%20Up :type Physics%20Handle%20Component%20Object%20Reference))
  (Variables|Default|SetPhysicsHandleRef PhysicsHandle%20Picking%20Up)
  (Variables|Default|SetHeld true)
  (Physics|SetEnableGravity (Variables|Default|GetStaticMesh) false)
  (Rendering|Material|SetMaterial (Variables|Default|GetStaticMesh) 0 "/Engine/VREditor/BasicMeshes/MI_Cube_02.MI_Cube_02"))

(fn CubeDropped
  (if (Variables|Default|GetHeld)
    (CallFunction|Swap-Collision true)
    (Utilities|IsValid (Variables|Default|GetPhysicsHandleRef)
      (:Is%20Valid
        (Variables|Default|SetHeld false)
        (Physics|SetEnableGravity (Variables|Default|GetStaticMesh) true)
        (Physics|Components|PhysicsHandle|ReleaseComponent (Variables|Default|GetPhysicsHandleRef))
        (Rendering|Material|SetMaterial (Variables|Default|GetStaticMesh) 0 "/Engine/VREditor/BasicMeshes/MI_Cube_03.MI_Cube_03")
        (return)))))

(fn AttachCloneCubetoClone
  (params (Clone%20Ref :type BP%20First%20Person%20Character%20Object%20Reference))
  (bind _rifle_ref (Variables|/Game/FirstPerson/Blueprints/BP_FirstPersonCharacter.BP_FirstPersonCharacter_C|GetRifle%20Ref Clone%20Ref))
  (bind _physicshandle (Variables|/Game/FirstPerson/Blueprints/BP_Rifle.BP_Rifle_C|GetPhysicsHandle _rifle_ref))
  (Utilities|IsValid Clone%20Ref
    (:Is%20Valid
      (Physics|Components|PhysicsHandle|GrabComponentatLocationwithRotation _physicshandle (Variables|Default|GetStaticMesh) "None" (Transformation|GetActorLocation) (Transformation|GetActorRotation))
      (CallFunction|CubePickedUp _physicshandle))))

(fn Enable/DisableShadows
  (params (Enable :type Boolean))
  (Rendering|SetCastShadow (Variables|Default|GetStaticMesh) Enable))

(fn DestroyCloneCube
  (params (Key :type B-Portal%20Object%20Reference%20%28by%20ref%29))
  (if (.ReturnValue (Utilities|Map|Find (Variables|/Game/Blueprints/PC-Portal.PC-Portal_C|GetPortal-Cube-Clones (Variables|Default|GetAs%20PC-Portal)) Key))
    (Utilities|Map|Remove (Variables|/Game/Blueprints/PC-Portal.PC-Portal_C|GetPortal-Cube-Clones (Variables|Default|GetAs%20PC-Portal)) Key)
    (else
      (Actor|DestroyActor))))