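; Floor puzzle button that the first-person character or companion cube holds down to validate connected cable paths.
; Overlaps fill a list of occupants; a timeline lowers the button and reverses once the list empties.
; A completed press marks linked BPSplines valid and turns the pad's dynamic material green, while release invalidates them and restores yellow.
; On BeginPlay it auto-links any spline with an endpoint near the button.
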(event OnComponentBeginOverlap(Detect)
  (params (OverlappedComponent :type Primitive%20Component%20Object%20Reference) (OtherActor :type Actor%20Object%20Reference) (OtherComp :type Primitive%20Component%20Object%20Reference) (OtherBodyIndex :type Integer) (bFromSweep :type Boolean) (SweepResult :type Hit%20Result%20Structure%20%28by%20ref%29))
  (bind _asbp_first_person_character (Utilities|Casting|CastToBP_FirstPersonCharacter OtherActor)
    (:then
      (CallFunction|ObjectonButton _asbp_first_person_character))
    (:CastFailed
      (bind _asgrabbable_small_cube (Utilities|Casting|CastToBP-CompanionCube OtherActor))
      (CallFunction|ObjectonButton _asgrabbable_small_cube))))

(event OnComponentEndOverlap(Detect)
  (params (OverlappedComponent :type Primitive%20Component%20Object%20Reference) (OtherActor :type Actor%20Object%20Reference) (OtherComp :type Primitive%20Component%20Object%20Reference) (OtherBodyIndex :type Integer))
  (bind _asbp_first_person_character (Utilities|Casting|CastToBP_FirstPersonCharacter OtherActor)
    (:then
      (CallFunction|ObjectOffButton _asbp_first_person_character))
    (:CastFailed
      (bind _asgrabbable_small_cube (Utilities|Casting|CastToBP-CompanionCube OtherActor))
      (CallFunction|ObjectOffButton _asgrabbable_small_cube))))

(event Custom|Button%20Pressed
  ;[1 1 1] Button Movement
  (bind (_direction _alpha) (Timeline|TL-ButtonPressed Play)
    (:Update
      (Transformation|SetRelativeLocation (Variables|Default|GetSM-Button) (Math|Vector|Lerp(Vector) "0, 0,10.000000" "0, 0,-5.000000" _alpha) false false))
    (:Finished
      (switch Utilities|FlowControl|Switch|SwitchonETimelineDirection _direction
        (:Forward
          (Variables|Default|SetButton%20Down true)
          (CallFunction|PuzzleComplete))))))

(event Custom|Button%20Released
  ;[1 1 1] Button Movement
  (Variables|Default|SetButton%20Down false)
  (CallFunction|PuzzleIncomplete)
  (bind (_direction _alpha) (Timeline|TL-ButtonPressed Reverse)
    (:Update
      (Transformation|SetRelativeLocation (Variables|Default|GetSM-Button) (Math|Vector|Lerp(Vector) "0, 0,10.000000" "0, 0,-5.000000" _alpha) false false))
    (:Finished
      (switch Utilities|FlowControl|Switch|SwitchonETimelineDirection _direction
        (:Forward
          (Variables|Default|SetButton%20Down true)
          (CallFunction|PuzzleComplete))))))

(event EventBeginPlay
  (Components|Timeline|SetPlayRate (Variables|Default|GetTL-ButtonPressed) 1.0)
  (bind _returnvalue (Rendering|Material|CreateDynamicMaterialInstance "/Game/Assets/Material/MI_Cables.MI_Cables" "None" "None" :!class /Script/Engine.KismetMaterialLibrary))
  (Variables|Default|SetMaterial _returnvalue)
  (Rendering|Material|SetVectorParameterValue (Variables|Default|GetMaterial) "GridColor" "(R=1.000000,G=1.000000,B=0.000000,A=1.000000)" :!class /Script/Engine.MaterialInstanceDynamic)
  (Rendering|Material|SetMaterial (Variables|Default|GetSM-Pad) 0 (Variables|Default|GetMaterial))
  (CallFunction|GetLinesAttached))

(fn ConstructionScript)

(fn ObjectonButton
  (params (Actor%20On :type Actor%20Object%20Reference))
  (Utilities|Array|AddUnique (Variables|Default|GetActors%20Overlapping) Actor%20On)
  (if (not (Variables|Default|GetButton%20Down))
    (CallFunction|ButtonPressed)))

(fn ObjectOffButton
  (params (Actor%20Off :type Actor%20Object%20Reference))
  (Utilities|Array|RemoveItem (Variables|Default|GetActors%20Overlapping) Actor%20Off)
  (if (== (Utilities|Array|Length (Variables|Default|GetActors%20Overlapping)) 0)
    (CallFunction|ButtonReleased)))

(fn PuzzleComplete
  (for _array_element (Variables|Default|GetSpline%20Connected)
    (Default|PathValid _array_element true))
  (Rendering|Material|SetVectorParameterValue (Variables|Default|GetMaterial) "GridColor" "(R=0.000000,G=1.000000,B=0.000000,A=1.000000)" :!class /Script/Engine.MaterialInstanceDynamic))

(fn PuzzleIncomplete
  (for _array_element (Variables|Default|GetSpline%20Connected)
    (Default|PathValid _array_element false))
  (Rendering|Material|SetVectorParameterValue (Variables|Default|GetMaterial) "GridColor" "(R=1.000000,G=1.000000,B=0.000000,A=1.000000)" :!class /Script/Engine.MaterialInstanceDynamic))

(fn GetLinesAttached
  (bind _outactors (Actor|GetAllActorsOfClass "/Game/Blueprints/Puzzles/BP-Spline.BP-Spline_C"))
  (for _array_element _outactors
    (if (or (< (Math|Vector|Distance(Vector) (Transformation|GetActorLocation) (.Start (Default|GetFirstandLastPoint _array_element))) 1.2e+02) (< (Math|Vector|Distance(Vector) (.End (Default|GetFirstandLastPoint _array_element)) (Transformation|GetActorLocation)) 1.2e+02))
      (Utilities|Array|AddUnique (Variables|Default|GetSpline%20Connected) _array_element))))