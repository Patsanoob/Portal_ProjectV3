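; Puzzle cube spawner that drops in a companion cube and animates its ring of door meshes.
; SpawnCube runs two seconds after BeginPlay, spawning a scaled BPCompanionCube at an offset relative to the spawner's transform.
; It then plays a timeline from the start, whose alpha lerps the roll of eight door meshes to swing them, preserving their pitch and yaw.
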(event Custom|Spawn%20Cube
  (Game|SpawnActorfromClass "/Game/Blueprints/Puzzles/BP-CompanionCube.BP-CompanionCube_C" (Math|Transform|MakeTransform (Math|Transform|TransformLocation (Transformation|GetActorTransform) "0, 0,-50.000000") (Math|Transform|TransformRotation (Transformation|GetActorTransform) "50.000000, 0, 0") "1.800000,1.800000,1.800000") "Undefined" 0 self 0)
  (bind _alpha (Timeline|TL-Cube%20Spawned PlayFromStart)
    (:Update
      (for _array_element (Utilities|Array|MakeArray (Variables|Default|GetSM-Door4) (Variables|Default|GetSM-Door6) (Variables|Default|GetSM-Door3) (Variables|Default|GetSM-Door2) (Variables|Default|GetSM-Door1) (Variables|Default|GetSM-Door5) (Variables|Default|GetSM-Door8) (Variables|Default|GetSM-Door7))
        (Transformation|SetRelativeRotation _array_element (Math|Rotator|MakeRotator (Math|Float|Lerp 0.0 7e+01 _alpha) (.pitch (Variables|/Script/Engine.SceneComponent|GetRelativeRotation _array_element)) (.yaw (Variables|/Script/Engine.SceneComponent|GetRelativeRotation _array_element))) false false)))))

(event EventBeginPlay
  (Utilities|FlowControl|Delay 2.0)
  (CallFunction|SpawnCube))

(event Collision|EventActorBeginOverlap
  (params (OtherActor :type Actor%20Object%20Reference)))

(event EventTick
  (params (DeltaSeconds :type Float%20%28single-precision%29)))

(fn ConstructionScript)