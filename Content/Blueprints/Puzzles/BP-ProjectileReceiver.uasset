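; BP-ProjectileReceiver is a puzzle receiver actor whose cable material turns from yellow to green when PuzzleComplete is called.
; On BeginPlay it collects every BPSpline with an endpoint near it and moves its SpotLight just short of the surface hit by an upward trace, destroying the light if nothing is hit.
; PuzzleComplete marks the connected splines as valid paths, recolors the dynamic material and removes the SpotLight.
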(event EventBeginPlay
  (bind _returnvalue (Transformation|GetActorLocation))
  (CallFunction|GetLinesAttached)
  (bind (_outhit _returnvalue_2) (Collision|LineTraceByChannel _returnvalue (+ _returnvalue (* (Transformation|GetActorUpVector) 7e+03)) "TraceTypeQuery1" false 0 "ForDuration"))
  (if _returnvalue_2
    (Transformation|SetWorldLocation (Variables|Default|GetSpotLight) (+ (.ImpactPoint (Collision|BreakHitResult _outhit)) (* (Transformation|GetActorUpVector) -5e+01)) false false)
    (else
      (Components|DestroyComponent (Variables|Default|GetSpotLight)))))

(fn ConstructionScript
  (bind _returnvalue (Rendering|Material|CreateDynamicMaterialInstance "/Game/Assets/Material/MI_Cables.MI_Cables" "None" "None" :!class /Script/Engine.KismetMaterialLibrary))
  (bind _output_get (Variables|Default|SetMaterial _returnvalue))
  (Rendering|Material|SetVectorParameterValue _output_get "GridColor" "(R=1.000000,G=1.000000,B=0.000000,A=1.000000)" :!class /Script/Engine.MaterialInstanceDynamic)
  (Rendering|Material|SetMaterial (Variables|Default|GetStaticMesh) 0 (Variables|Default|GetMaterial)))

(fn PuzzleComplete
  (for _array_element (Variables|Default|GetSpline%20Connected)
    (Default|PathValid _array_element true))
  (Rendering|Material|SetVectorParameterValue (Variables|Default|GetMaterial) "GridColor" "(R=0.000000,G=1.000000,B=0.000000,A=1.000000)" :!class /Script/Engine.MaterialInstanceDynamic)
  (Components|DestroyComponent (Variables|Default|GetSpotLight)))

(fn GetLinesAttached
  (bind _outactors (Actor|GetAllActorsOfClass "/Game/Blueprints/Puzzles/BP-Spline.BP-Spline_C"))
  (for _array_element _outactors
    (if (or (< (Math|Vector|Distance(Vector) (Transformation|GetActorLocation) (.Start (Default|GetFirstandLastPoint _array_element))) 1e+02) (< (Math|Vector|Distance(Vector) (.End (Default|GetFirstandLastPoint _array_element)) (Transformation|GetActorLocation)) 1e+02))
      (Utilities|Array|AddUnique (Variables|Default|GetSpline%20Connected) _array_element))))