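; Puzzle spawner actor that launches an energy projectile on BeginPlay and can spawn more on request until it is completed.
; Spawn_Energy waits a given delay, spawns BPEnergyProjectile above the actor with a reference back to the spawner, and stores it.
; The construction script gives the mesh a red dynamic cable material.
; ShutdownSpawner sets Complete to block further spawn requests and dims that material's grid color and intensity.
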(event Custom|Spawn_Energy
  (params (Delay :type Float%20%28double-precision%29))
  (if (not (Variables|Default|GetComplete))
    (Utilities|FlowControl|Delay Delay)
    (bind _returnvalue (Game|SpawnActorfromClass "/Game/Blueprints/Puzzles/BP-EnergyProjectile.BP-EnergyProjectile_C" (Math|Transform|MakeTransform (Math|Transform|TransformLocation (Transformation|GetActorTransform) "0, 0,120.000000") (Math|Transform|TransformRotation (Transformation|GetActorTransform) "0, 0, 0") "1.000000,1.000000,1.000000") "Undefined" 0 self 0))
    (Variables|Default|SetEnergyBall-Ref _returnvalue)))

(event EventBeginPlay
  (CallFunction|SpawnEnergy 0.0))

(fn ConstructionScript
  (bind _returnvalue (Rendering|Material|CreateDynamicMaterialInstance "/Game/Assets/Material/MI_Cables.MI_Cables" "None" "None" :!class /Script/Engine.KismetMaterialLibrary))
  (bind _output_get (Variables|Default|SetMaterial _returnvalue))
  (Rendering|Material|SetVectorParameterValue _output_get "GridColor" "(R=1.000000,G=0.000000,B=0.000000,A=1.000000)" :!class /Script/Engine.MaterialInstanceDynamic)
  (Rendering|Material|SetMaterial (Variables|Default|GetSM-Spawner) 0 (Variables|Default|GetMaterial)))

(fn ShutdownSpawner
  (bind _material (Variables|Default|GetMaterial))
  (Variables|Default|SetComplete true)
  (Rendering|Material|SetVectorParameterValue _material "GridColor" "(R=0.005208,G=0.000000,B=0.000000,A=1.000000)" :!class /Script/Engine.MaterialInstanceDynamic)
  (Rendering|Material|SetScalarParameterValue _material "Intensity Min" 0.0 :!class /Script/Engine.MaterialInstanceDynamic)
  (Rendering|Material|SetScalarParameterValue _material "Intensity Max" 2.0 :!class /Script/Engine.MaterialInstanceDynamic))