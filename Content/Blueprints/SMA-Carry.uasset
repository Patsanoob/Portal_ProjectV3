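; Physics prop that the first-person character's rifle can grab and carry through a physics handle.
; ManualAttach grabs the mesh at its location, marks it held and sets the rifle to ignore walls.
; ReleaseGun drops any grabbed component and clears the held flag and rifle reference, leaving the wall setting untouched.
; Every tick, it rewrites the mesh's linear velocity to cap its speed, whether held or not.
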(event EventTick
  (params (DeltaSeconds :type Float%20%28single-precision%29))
  (bind _returnvalue (Transformation|GetVelocity))
  (Physics|SetPhysicsLinearVelocity (Variables|Debug|GetStaticMeshComponent) (* (Math|Float|Clamp(Float) (Math|Vector|VectorLength _returnvalue) -8e+02 8e+02) (Math|Vector|Normalize _returnvalue)) false "None"))

(fn ConstructionScript)

(fn ManualAttach
  (params (First%20Person%20Ref :type BP%20First%20Person%20Character%20Object%20Reference))
  (bind _output_get (LocalVariables|SetL-FPS First%20Person%20Ref))
  (bind _output_get_2 (Variables|Default|SetAs-BP_Rifle (Variables|/Game/FirstPerson/Blueprints/BP_FirstPersonCharacter.BP_FirstPersonCharacter_C|GetRifle%20Ref _output_get)))
  (Physics|Components|PhysicsHandle|GrabComponentatLocationwithRotation (Variables|/Game/FirstPerson/Blueprints/BP_Rifle.BP_Rifle_C|GetPhysicsHandle _output_get_2) (Variables|Debug|GetStaticMeshComponent) "None" (Transformation|GetWorldLocation (Variables|Debug|GetStaticMeshComponent)) "0, 0, 0")
  (Variables|Default|SetHeld true)
  (Variables|/Game/FirstPerson/Blueprints/BP_Rifle.BP_Rifle_C|SetIgnore%20Walls (Variables|/Game/FirstPerson/Blueprints/BP_FirstPersonCharacter.BP_FirstPersonCharacter_C|GetRifle%20Ref (LocalVariables|GetL-FPS)) true))

(fn ReleaseGun
  (bind _as_bp_rifle (Variables|Default|GetAs-BP_Rifle)
    (:then
      (Utilities|IsValid (Class|PhysicsHandleComponent|GetGrabbedComponent (Variables|/Game/FirstPerson/Blueprints/BP_Rifle.BP_Rifle_C|GetPhysicsHandle _as_bp_rifle))
        (:Is%20Valid
          (Variables|Default|SetHeld false)
          (Physics|Components|PhysicsHandle|ReleaseComponent (Variables|/Game/FirstPerson/Blueprints/BP_Rifle.BP_Rifle_C|GetPhysicsHandle _as_bp_rifle))
          (Variables|Default|SetAs-BP_Rifle 0))))
    (:else)))