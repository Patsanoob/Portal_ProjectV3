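; BP-Surface_Portal is an actor that builds a flat or ramped surface from a Corner vector, with no active gameplay logic.
; The construction script scales SMSurface in X and Y on a 200-unit basis, using Corner's X and Y directly when its Z is zero.
; For ramps, it takes the Y-Z hypotenuse as length and rolls the mesh by the negated arctangent of Z over Y.
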(event EventBeginPlay
  (|CallParentFunction) ; This node is disabled and will not be called.\nDrag off pins to build functionality.
)

(event Collision|EventActorBeginOverlap
  (params (OtherActor :type Actor%20Object%20Reference))
  (|CallParentFunction OtherActor) ; This node is disabled and will not be called.\nDrag off pins to build functionality.
)

(event EventTick
  (params (DeltaSeconds :type Float%20%28single-precision%29))
  (|CallParentFunction DeltaSeconds) ; This node is disabled and will not be called.\nDrag off pins to build functionality.
)

(fn ConstructionScript
  (bind _corner (Variables|Default|GetCorner))
  (bind _corner_2 (Variables|Default|GetCorner))
  (bind _corner_3 (Variables|Default|GetCorner))
  (bind _returnvalue (/ _corner 2e+02))
  (|CallParentFunction)
  (if (== (.z (Variables|Default|GetCorner)) 0.0)
    ;[1 1 1] Set Appropriate Scale (If Flat)
    (Transformation|SetRelativeScale3D (Variables|Default|GetSM-Surface) (Math|Vector|MakeVector (.x _returnvalue) (.y _returnvalue) 1.0))
    (else
      ;[1 1 1] Set Appropriate Scale (If Ramp)
      (Transformation|SetRelativeScale3D (Variables|Default|GetSM-Surface) (Math|Vector|MakeVector (.x (/ (Variables|Default|GetCorner) 2e+02)) (/ (Math|Float|Sqrt (+ (Math|Float|Square (.y _corner_3)) (Math|Float|Square (.z _corner_3)))) 2e+02) 1.0))
      ;[1 1 1] Set Actor Rotation
      (Transformation|SetRelativeRotation (Variables|Default|GetSM-Surface) (Math|Rotator|MakeRotator (* (Class|KismetMathLibrary|DegAtan (/ (.z _corner_2) (.y _corner_2))) -1.0) 0.0 0.0) false false))))