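; Level-design actor that spawns a moving B_Plat platform from editable waypoints, behaviour type, duration and size, auto-activating it unless flagged as Puzzle.
; Waypoints become world-offset control points, with the actor's origin appended for LoopReset.
; Flat multi-point paths get instanced pillars in the construction script and Niagara laser beams at BeginPlay.
; It binds to nearby BPSpline endpoints, though LineChanged is empty; Active calls the platform's stop/start.
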(event Custom|Active
  (Default|Stop-StartMovement (Variables|Default|GetPlatform) (Variables|Default|GetDuration)))

(event EventBeginPlay
  (bind _size (Variables|Default|GetSize))
  (bind _returnvalue (/ _size 1e+02))
  (CallFunction|GetLinesAttached)
  (bind _returnvalue_2 (Game|SpawnActorfromClass "/Game/Blueprints/LevelDesign/B_Plat.B_Plat_C" (Transformation|GetActorTransform) "Undefined" 0 (Variables|Default|GetInitial%20Delay) (CallFunction|CreateControlPoints) (Variables|Default|GetBehaviour%20Type) (Variables|Default|GetDuration) 0))
  (Variables|Default|SetPlatform _returnvalue_2)
  (Transformation|SetRelativeScale3D (Variables|/Game/Blueprints/LevelDesign/B_Plat.B_Plat_C|GetPlatform (Variables|Default|GetPlatform)) (Math|Vector|MakeVector _returnvalue _returnvalue 1.0))
  (Utilities|FlowControl|Sequence
    (:then_0
      (if (CallFunction|SpawnLaser (Variables|Default|GetLocations))
        (CallFunction|SpawnLasers)))
    (:then_1
      (if (not (Variables|Default|GetPuzzle?))
        (Default|Activate (Variables|Default|GetPlatform))))))

(fn ConstructionScript
  (Utilities|FlowControl|Sequence
    (:then_0
      ;[1 1 1] Change Location of new location Spot
      (if (and (!= 0 (Utilities|Array|LastIndex (Variables|Default|GetLocations))) (Class|KismetMathLibrary|EqualExactlyVectorVector (Utilities|Array|Get(acopy) (Variables|Default|GetLocations) (Utilities|Array|LastIndex (Variables|Default|GetLocations))) "0, 0, 0"))
        (Utilities|Array|SetArrayElem (Variables|Default|GetLocations) (Utilities|Array|LastIndex (Variables|Default|GetLocations)) (Utilities|Array|Get(acopy) (Variables|Default|GetLocations) (- (Utilities|Array|LastIndex (Variables|Default|GetLocations)) 1)))))
    (:then_1
      (if (CallFunction|SpawnLaser (Variables|Default|GetLocations))
        (for _array_element (Variables|Default|GetLocations)
          (Components|InstancedStaticMesh|AddInstance (Variables|Default|GetISM-Pillars) (Math|Transform|MakeTransform _array_element) false))))))

(fn CreateControlPoints
  (for _array_element (Variables|Default|GetLocations)
    (Utilities|Array|Add (LocalVariables|GetReturn%20Array) (Utilities|Struct|MakeInterpControlPoint (+ _array_element (Transformation|GetActorLocation)) false)))
  (if (Utilities|Enum|Equal(Enum) (Variables|Default|GetBehaviour%20Type) "Loop_Reset")
    (Utilities|Array|Add (LocalVariables|GetReturn%20Array) (Utilities|Struct|MakeInterpControlPoint (Transformation|GetActorLocation) false))
    (return (LocalVariables|GetReturn%20Array))
    (else
      (return (LocalVariables|GetReturn%20Array)))))

(fn SpawnLaser
  (params (InputPin :type Array%20of%20Vectors))
  (if (> (Utilities|Array|Length InputPin) 1)
    (for _array_element InputPin
      (if (!= (.Z (Math|Vector|BreakVector _array_element)) 0.0)
        (return false)))
    (return true)
    (else
      (return false))))

(fn SpawnLasers
  (bind _locations (Variables|Default|GetLocations))
  (for (_array_element _array_index) (Variables|Default|GetLocations)
    (LocalVariables|SetCurrent%20Location _array_element)
    (LocalVariables|SetIndex _array_index)
    (if (!= _array_index (Utilities|Array|LastIndex (Variables|Default|GetLocations)))
      (bind _returnvalue (Niagara|SpawnSystematLocation "/Game/Assets/Particle/NS-Laser.NS-Laser" (Math|Transform|TransformLocation (Transformation|GetActorTransform) (- (LocalVariables|GetCurrent%20Location) "0,0,90.000000"))))
      (Utilities|Array|AddUnique (Variables|Default|GetArray%20Of%20Particles) _returnvalue)
      (Effects|Components|ParticleSystem|SetVectorParameter _returnvalue "Beam End" (Math|Transform|TransformLocation (Transformation|GetActorTransform) (- (Utilities|Array|Get(acopy) (Variables|Default|GetLocations) (+ (LocalVariables|GetIndex) 1)) "0,0,90.000000")))))
  (if (Utilities|Enum|Equal(Enum) (Variables|Default|GetBehaviour%20Type) "Loop_Reset")
    (bind _returnvalue_2 (Niagara|SpawnSystematLocation "/Game/Assets/Particle/NS-Laser.NS-Laser" (Math|Transform|TransformLocation (Transformation|GetActorTransform) (- (Utilities|Array|Get(acopy) _locations (Utilities|Array|LastIndex _locations)) "0,0,90.000000"))))
    (Effects|Components|ParticleSystem|SetVectorParameter _returnvalue_2 "Beam End" (Math|Transform|TransformLocation (Transformation|GetActorTransform) (- (Utilities|Array|Get(acopy) (Variables|Default|GetLocations)) "0,0,90.000000")))))

(fn GetLinesAttached
  (bind _outactors (Actor|GetAllActorsOfClass "/Game/Blueprints/Puzzles/BP-Spline.BP-Spline_C"))
  (for _array_element _outactors
    (if (or (< (Math|Vector|Distance(Vector) (Transformation|GetActorLocation) (.Start (Default|GetFirstandLastPoint _array_element))) 2e+02) (< (Math|Vector|Distance(Vector) (.End (Default|GetFirstandLastPoint _array_element)) (Transformation|GetActorLocation)) 2e+02))
      (Utilities|Array|AddUnique (Variables|Default|GetSpline%20Connected) _array_element)
      (EventDispatchers|BindEventtoChangedState _array_element (EventDispatchers|CreateEvent :!event Custom|Active)))))

(fn LineChanged)