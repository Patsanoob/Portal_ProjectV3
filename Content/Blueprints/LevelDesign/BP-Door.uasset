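; Sliding double door for level design that opens or closes based on the state of connected spline cables.
; On BeginPlay it collects every BPSpline with an endpoint near the door and binds to its changed-state event.
; CanDoorOpen checks that all connected cables are valid, opening or closing the door accordingly.
; A timeline lerps both panels apart, reverses to close, and updates the Open flag when finished.
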(event Custom|Open%20Door
  (bind (_direction _alpha) (Timeline|TL-DoorOpen/Close Play)
    (:Update
      (Transformation|SetRelativeLocation (Variables|Default|GetDoorA) (Math|Vector|Lerp(Vector) "0.000000,50.000000,150.000000" "0,140.000000,150.000000" _alpha) false false)
      (Transformation|SetRelativeLocation (Variables|Default|GetDoorB) (Math|Vector|Lerp(Vector) "0,-50.000000,150.000000" "0.000000,-140.000000,150.000000" _alpha) false false))
    (:Finished
      (switch Utilities|FlowControl|Switch|SwitchonETimelineDirection _direction
        (:Forward
          (Variables|Default|SetOpen true))
        (:Backward
          (Variables|Default|SetOpen false))))))

(event Custom|Close%20Door
  (bind (_direction _alpha) (Timeline|TL-DoorOpen/Close Reverse)
    (:Update
      (Transformation|SetRelativeLocation (Variables|Default|GetDoorA) (Math|Vector|Lerp(Vector) "0.000000,50.000000,150.000000" "0,140.000000,150.000000" _alpha) false false)
      (Transformation|SetRelativeLocation (Variables|Default|GetDoorB) (Math|Vector|Lerp(Vector) "0,-50.000000,150.000000" "0.000000,-140.000000,150.000000" _alpha) false false))
    (:Finished
      (switch Utilities|FlowControl|Switch|SwitchonETimelineDirection _direction
        (:Forward
          (Variables|Default|SetOpen true))
        (:Backward
          (Variables|Default|SetOpen false))))))

(event EventBeginPlay
  (CallFunction|GetLinesAttached))

(fn ConstructionScript)

(fn CanDoorOpen
  (for _array_element (Variables|Default|GetSpline%20Connected)
    (if (not (Variables|/Game/Blueprints/Puzzles/BP-Spline.BP-Spline_C|GetValid%20Cable _array_element))
      (LocalVariables|SetReturn%20Value false)))
  (if (LocalVariables|GetReturn%20Value)
    (CallFunction|OpenDoor)
    (else
      (CallFunction|CloseDoor))))

(fn GetLinesAttached
  (bind _outactors (Actor|GetAllActorsOfClass "/Game/Blueprints/Puzzles/BP-Spline.BP-Spline_C"))
  (for _array_element _outactors
    (if (or (< (Math|Vector|Distance(Vector) (Transformation|GetActorLocation) (.Start (Default|GetFirstandLastPoint _array_element))) 2e+02) (< (Math|Vector|Distance(Vector) (.End (Default|GetFirstandLastPoint _array_element)) (Transformation|GetActorLocation)) 2e+02))
      (Utilities|Array|AddUnique (Variables|Default|GetSpline%20Connected) _array_element)
      (EventDispatchers|BindEventtoChangedState _array_element (EventDispatchers|CreateEvent :!event CanDoorOpen)))))