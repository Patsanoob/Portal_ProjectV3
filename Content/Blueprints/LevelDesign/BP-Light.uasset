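; BP-Light is a placeable level-design light panel that pairs an emissive decal with a Rect Light.
; The construction script feeds the exposed color and intensity to both the light and a dynamic M_LightDecal material, and sets the light's range and barn doors.
; Rect Light width and height follow actor scale, while its intensity is a multiple of the panel's emissive intensity.
; UpdateLight recolors both light and decal together.
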(event EventBeginPlay)

(event EventTick
  (params (DeltaSeconds :type Float%20%28single-precision%29)))

(fn ConstructionScript
  (bind _returnvalue (Transformation|GetActorScale3D))
  (bind _returnvalue_2 (Rendering|Material|CreateDynamicMaterialInstance "/Game/Assets/Material/M_LightDecal.M_LightDecal" "None" "None" :!class /Script/Engine.KismetMaterialLibrary))
  (Variables|Default|SetMaterial_Inst _returnvalue_2)
  ;[1 1 1] Setup Decal Parameters
  (Rendering|Material|SetVectorParameterValue (Variables|Default|GetMaterial_Inst) "Color" (Variables|Default|GetLight%20Color) :!class /Script/Engine.MaterialInstanceDynamic)
  (Rendering|Material|SetScalarParameterValue (Variables|Default|GetMaterial_Inst) "Intensity" (Variables|Default|GetEmissive%20Pannel%20Intensity) :!class /Script/Engine.MaterialInstanceDynamic)
  ;[1 1 1] Set Decal Material
  (Rendering|Components|Decal|SetDecalMaterial (Variables|Decal|GetDecal) (Variables|Default|GetMaterial_Inst))
  ;[1 1 1] Change Rect Light parameters based on Editor input
  (Rendering|Components|Light|SetIntensity (Variables|Default|GetRectLight) (* (Variables|Default|GetEmissive%20Pannel%20Intensity) 1e+03))
  (Rendering|Components|Light|SetLightColor (Variables|Default|GetRectLight) (Variables|Default|GetLight%20Color) true)
  (Rendering|Lighting|SetAttenuationRadius (Variables|Default|GetRectLight) (Variables|Default|GetRange))
  ;[1 1 1] Adjust size of rect light to scale
  (Class|RectLightComponent|SetSourceWidth (Variables|Default|GetRectLight) (* (.x _returnvalue) 2e+02))
  (Class|RectLightComponent|SetSourceHeight (Variables|Default|GetRectLight) (* (.y _returnvalue) 2e+02))
  (Class|RectLightComponent|SetBarnDoorAngle (Variables|Default|GetRectLight) (Variables|Default|GetBarnDoor%20Angle))
  (Class|RectLightComponent|SetBarnDoorLength (Variables|Default|GetRectLight) (Variables|Default|GetBarnDoor%20Length)))

(fn UpdateLight
  (params (Light%20Color :type Linear%20Color%20Structure))
  (Variables|Default|SetLight%20Color Light%20Color)
  (Rendering|Components|Light|SetLightColor (Variables|Default|GetRectLight) (Variables|Default|GetLight%20Color) true)
  (Rendering|Material|SetVectorParameterValue (Variables|Default|GetMaterial_Inst) "Color" (Variables|Default|GetLight%20Color) :!class /Script/Engine.MaterialInstanceDynamic)
  (Rendering|Components|Decal|SetDecalMaterial (Variables|Decal|GetDecal) (Variables|Default|GetMaterial_Inst)))