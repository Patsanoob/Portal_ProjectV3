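; BP-Window is a level design Blueprint for a window built from a Glass pane on top of a thin Bottom piece.
; Its construction script scales and positions both components from the Y and Z of the Height vector, anchored at the actor's origin.
; The Bottom keeps a fixed height while the Glass fills the remaining height above it.
; The event graph holds no active logic.
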(event EventBeginPlay)

(event Collision|EventActorBeginOverlap
  (params (OtherActor :type Actor%20Object%20Reference)))

(event EventTick
  (params (DeltaSeconds :type Float%20%28single-precision%29)))

(fn ConstructionScript
  (bind _height (Variables|Default|GetHeight))
  (bind _height_2 (Variables|Default|GetHeight))
  (Transformation|SetRelativeScale3D (Variables|Default|GetGlass) (Math|Vector|MakeVector 0.05 (/ (.y _height) 1e+02) (/ (- (.z _height) 1e+01) 1e+02)))
  (Transformation|SetRelativeLocation (Variables|Default|GetGlass) (Math|Vector|MakeVector 2.5 (/ (.y _height_2) 2.0) (+ (/ (- (.z _height_2) 1e+01) 2.0) 1e+01)) false false)
  (Transformation|SetRelativeScale3D (Variables|Default|GetBottom) (Math|Vector|MakeVector 0.05 (/ (.y (Variables|Default|GetHeight)) 1e+02) 0.1))
  (Transformation|SetRelativeLocation (Variables|Default|GetBottom) (Math|Vector|MakeVector 2.5 (/ (.y (Variables|Default|GetHeight)) 2.0) 5.0) false false))