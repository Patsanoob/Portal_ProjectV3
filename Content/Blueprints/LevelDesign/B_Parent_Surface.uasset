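; Parent level-design Blueprint that builds a Floor or Ramp block from a Corner vector.
; The construction script rounds Corner and the actor transform, then moves and scales 200-unit mesh pieces and destroys unused ones.
; Floors get side walls unless height is zero; ramps tilt the surface along the hypotenuse and add triangle sides, underside and back wall.
; UpdateCollisionResponse sets a channel response across the pieces used by each type.
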(event EventBeginPlay)

(event Collision|EventActorBeginOverlap
  (params (OtherActor :type Actor%20Object%20Reference)))

(event EventTick
  (params (DeltaSeconds :type Float%20%28single-precision%29)))

(fn ConstructionScript
  (Variables|Default|SetCorner (Math|Vector|MakeVector (Math|Conversions|ToFloat(Integer) (Math|Float|Round (.x (Variables|Default|GetCorner)))) (Math|Conversions|ToFloat(Integer) (Math|Float|Round (.y (Variables|Default|GetCorner)))) (Math|Conversions|ToFloat(Integer) (Math|Float|Round (.z (Variables|Default|GetCorner))))))
  (Transformation|SetActorLocation (|RoundLocation) false false)
  (Transformation|SetActorRotation (|RoundRotation))
  (switch Utilities|FlowControl|Switch|SwitchonE-TypeOfFloor (Variables|Default|GetType)
    (:NewEnumerator0
      ;[1 1 1] Remove Triangles
      (Components|DestroyComponent (Variables|Default|GetSM_Triangle-L))
      (|CollapsedScale)
      (if (CallFunction|ShowWalls)
        (Variables|Default|SetCorner (Math|Vector|MakeVector (.x (Variables|Default|GetCorner)) (.y (Variables|Default|GetCorner)) 0.0))
        (Components|DestroyComponent (Variables|Default|GetSM-Wall_Up))
        (else
          (Transformation|SetRelativeLocation (Variables|Default|GetSM_Surface) (Math|Vector|MakeVector 0.0 0.0 (.z (Variables|Default|GetCorner))) false false)
          ;[1 1 1] Update Locations of walls that need to move
          (Transformation|SetRelativeLocation (Variables|Default|GetSM-Wall_Up) (Math|Vector|MakeVector (.x (Variables|Default|GetCorner)) 0.0 0.0) false false)
          (Transformation|SetRelativeLocation (Variables|Default|GetSM-Wall_Right) (Math|Vector|MakeVector 0.0 (.y (Variables|Default|GetCorner)) 0.0) false false)
          ;[1 1 1] Set Location On the Z
          (Transformation|AddLocalOffset (Variables|Default|GetSM-Wall_Left) "0, 0, 0" false false)
          (Transformation|AddLocalOffset (Variables|Default|GetSM-Wall_Left) (Math|Vector|MakeVector 0.0 (* (.z (Variables|Default|GetCorner)) -1.0) 0.0) false false)
          (Transformation|AddLocalOffset (Variables|Default|GetSM-Wall_Up) (Math|Vector|MakeVector (* (.z (Variables|Default|GetCorner)) -1.0) 0.0 0.0) false false)
          ;[1 1 1] Set Relative Scale For Left Wall
          (Transformation|SetRelativeScale3D (Variables|Default|GetSM-Wall_Left) (Math|Vector|MakeVector (/ (.y (Variables|Default|GetCorner)) 2e+02) (/ (.z (Variables|Default|GetCorner)) 2e+02) 1.0))
          ;[1 1 1] Set Relative Scale For Right Wall
          (Transformation|SetRelativeScale3D (Variables|Default|GetSM-Wall_Right) (Math|Vector|MakeVector (/ (.x (Variables|Default|GetCorner)) 2e+02) (/ (.z (Variables|Default|GetCorner)) 2e+02) 1.0))
          ;[1 1 1] Set Relative Scale For Up Wall
          (Transformation|SetRelativeScale3D (Variables|Default|GetSM-Wall_Up) (Math|Vector|MakeVector (/ (.z (Variables|Default|GetCorner)) 2e+02) (/ (.y (Variables|Default|GetCorner)) 2e+02) 1.0))
          ;[1 1 1] Set Relative Scale For Down Wall
          (Transformation|SetRelativeScale3D (Variables|Default|GetSM-Wall_Down) (Math|Vector|MakeVector (/ (.z (Variables|Default|GetCorner)) 2e+02) (/ (.x (Variables|Default|GetCorner)) 2e+02) 1.0)))))
    (:NewEnumerator1
      ;[1 1 1] Set Scale Relative To Corner
      (Transformation|SetRelativeScale3D (Variables|Default|GetSM_Surface) (Math|Vector|MakeVector (.x (/ (Variables|Default|GetCorner) 2e+02)) (|CalculateLengthOfHypotenuse) 1.0))
      ;[1 1 1] Set Location
      (Transformation|SetRelativeLocation (Variables|Default|GetSM_Under) (Math|Vector|MakeVector (.x (Variables|Default|GetCorner)) 0.0 0.0) false false)
      ;[1 1 1] Set Scale Of Under
      (Transformation|SetRelativeScale3D (Variables|Default|GetSM_Under) (Math|Vector|MakeVector (.x (/ (Variables|Default|GetCorner) 2e+02)) (.y (/ (Variables|Default|GetCorner) 2e+02)) 1.0))
      ;[1 1 1] Set Floor Relative Rotation
      (Transformation|SetRelativeRotation (Variables|Default|GetSM_Surface) (Math|Rotator|MakeRotator (* (Class|KismetMathLibrary|DegAtan (/ (.z (Variables|Default|GetCorner)) (.y (Variables|Default|GetCorner)))) -1.0) 0.0 0.0) false false)
      (Variables|Default|SetAngle (* (Class|KismetMathLibrary|DegAtan (/ (.z (Variables|Default|GetCorner)) (.y (Variables|Default|GetCorner)))) -1.0))
      ;[1 1 1] Spawn Side 1
      (Transformation|SetRelativeTransform (Variables|Default|GetSM_Triangle-L) (Math|Transform|MakeTransform (Math|Vector|MakeVector 0.0 (.y (Variables|Default|GetCorner)) 0.0) "0, 0, 0" (Math|Vector|MakeVector 1.0 (.y (/ (Variables|Default|GetCorner) 2e+02)) (.z (/ (Variables|Default|GetCorner) 2e+02)))) false false)
      ;[1 1 1] Spawn Side 2
      (Transformation|SetRelativeTransform (Variables|Default|GetSM_Triangle-R) (Math|Transform|MakeTransform (Math|Vector|MakeVector (.x (Variables|Default|GetCorner)) (.y (Variables|Default|GetCorner)) 0.0) "0, 0, 0" (Math|Vector|MakeVector 1.0 (.y (/ (Variables|Default|GetCorner) 2e+02)) (.z (/ (Variables|Default|GetCorner) 2e+02)))) false false)
      (Components|DestroyComponent (Variables|Default|GetSM-Wall_Down))
      (Transformation|SetRelativeLocation (Variables|Default|GetSM-Wall_Right) (Math|Vector|MakeVector 0.0 (.y (Variables|Default|GetCorner)) (.z (Variables|Default|GetCorner))) false false)
      (Transformation|SetRelativeScale3D (Variables|Default|GetSM-Wall_Right) (Math|Vector|MakeVector (/ (.x (Variables|Default|GetCorner)) 2e+02) (/ (.z (Variables|Default|GetCorner)) 2e+02) 1.0)))))

(fn ShowWalls
  (return (Math|Float|NearlyEqual(Float) (.z (Variables|Default|GetCorner)) 0.0 1e-06)))

(fn UpdateCollisionResponse
  (params (Channel :type ECollisionChannel%20Enum :default "ECC_WorldStatic") (New%20Response :type ECollisionResponse%20Enum :default "ECR_Ignore"))
  (Collision|SetCollisionResponsetoChannel (Variables|Default|GetSM_Surface) Channel New%20Response)
  (switch Utilities|FlowControl|Switch|SwitchonE-TypeOfFloor (Variables|Default|GetType)
    (:NewEnumerator0
      (if (not (CallFunction|ShowWalls))
        (Collision|SetCollisionResponsetoChannel (Variables|Default|GetSM-Wall_Down) Channel New%20Response)))
    (:NewEnumerator1
      (Collision|SetCollisionResponsetoChannel (Variables|Default|GetSM_Under) Channel New%20Response))))