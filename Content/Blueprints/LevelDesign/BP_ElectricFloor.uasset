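; BP_ElectricFloor is a level-design hazard floor that kills the first-person character and destroys companion cubes on contact.
; A TriggerVolume overlap casts the other actor and calls Death on the player or CubeDestroyed on a cube.
; The construction script runs its parent's, strips the under, wall and triangle mesh components, then centers and sizes the thin trigger box from the Corner vector.
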(event OnComponentBeginOverlap(Trigger-Volume)
  (params (OverlappedComponent :type Primitive%20Component%20Object%20Reference) (OtherActor :type Actor%20Object%20Reference) (OtherComp :type Primitive%20Component%20Object%20Reference) (OtherBodyIndex :type Integer) (bFromSweep :type Boolean) (SweepResult :type Hit%20Result%20Structure%20%28by%20ref%29))
  (bind _asbp_first_person_character (Utilities|Casting|CastToBP_FirstPersonCharacter OtherActor)
    (:then
      (Default|Death _asbp_first_person_character))
    (:CastFailed
      (bind _asbp_companion_cube (Utilities|Casting|CastToBP-CompanionCube OtherActor))
      (Default|CubeDestroyed _asbp_companion_cube))))

(event EventBeginPlay
  (|CallParentFunction) ; This node is disabled and will not be called.\nDrag off pins to build functionality.
)

(event Collision|EventActorBeginOverlap
  (params (OtherActor :type Actor%20Object%20Reference))
  (|CallParentFunction OtherActor) ; This node is disabled and will not be called.\nDrag off pins to build functionality.
)

(event EventTick
  (params (DeltaSeconds :type Float%20%28single-precision%29))
  (|CallParentFunction DeltaSeconds) ; This node is disabled and will not be called.\nDrag off pins to build functionality.
)

(fn ConstructionScript
  (bind _corner (Variables|Default|GetCorner))
  (bind _corner_2 (Variables|Default|GetCorner))
  (bind _returnvalue (/ _corner_2 2.0))
  (bind _returnvalue_2 (/ _corner 2.0))
  (|CallParentFunction)
  (Components|DestroyComponent (Variables|Default|GetSM_Under))
  ;[1 1 1] Set Location
  (Transformation|SetRelativeLocation (Variables|Default|GetTrigger-Volume) (Math|Vector|MakeVector (.x _returnvalue) (.y _returnvalue) 5.0) false false)
  (Components|Box|SetBoxExtent (Variables|Default|GetTrigger-Volume) (Math|Vector|MakeVector (.x _returnvalue_2) (.y _returnvalue_2) 1e+01) true))