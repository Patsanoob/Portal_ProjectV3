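; Level-transition elevator that is either an arrival or an exit, depending on whether NextLevelName is set.
; Without a name, it removes its trigger boxes and opens on BeginPlay, fading its child BP-Light from blue to white.
; With one, BoxEnter opens the doors and BoxInside closes them and fades the light back.
; It then saves the player's elevator-relative transform and level progress to GI-Portal and opens the level from DTLevels.
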(event OnComponentBeginOverlap(Box-Enter)
  (params (OverlappedComponent :type Primitive%20Component%20Object%20Reference) (OtherActor :type Actor%20Object%20Reference) (OtherComp :type Primitive%20Component%20Object%20Reference) (OtherBodyIndex :type Integer) (bFromSweep :type Boolean) (SweepResult :type Hit%20Result%20Structure%20%28by%20ref%29))
  (Utilities|Casting|CastToBP_FirstPersonCharacter OtherActor)
  (CallFunction|OpenDoors false))

(event OnComponentBeginOverlap(Box-Inside)
  (params (OverlappedComponent :type Primitive%20Component%20Object%20Reference) (OtherActor :type Actor%20Object%20Reference) (OtherComp :type Primitive%20Component%20Object%20Reference) (OtherBodyIndex :type Integer) (bFromSweep :type Boolean) (SweepResult :type Hit%20Result%20Structure%20%28by%20ref%29))
  (Utilities|Casting|CastToBP_FirstPersonCharacter OtherActor)
  (CallFunction|CloseDoors)
  (Components|DestroyComponent (Variables|Default|GetBox-Inside)))

(event Custom|Open%20Doors
  (params (Spawn :type Boolean))
  (Utilities|FlowControl|Sequence
    (:then_0
      (Components|MoveComponentTo (Variables|Default|GetDoor%202) "-100.000000, 0, 0" "0, 0, 0" false false 0.5 false))
    (:then_1
      (Components|MoveComponentTo (Variables|Default|GetDoor%201) "100.000000, 0, 0" "0, 0, 0" false false 0.5 false))
    (:then_2
      (if Spawn
        (bind _alpha (Timeline|TL-Open PlayFromStart)
          (:Update
            (bind _asbp_light (Utilities|Casting|CastToBP-Light (Variables|/Script/Engine.ChildActorComponent|GetChildActor (Variables|Default|GetLight))))
            (Default|UpdateLight _asbp_light (Math|Color|Lerp(LinearColor) "(R=0.000000,G=0.502886,B=1.000000,A=1.000000)" "(R=1.000000,G=1.000000,B=1.000000,A=1.000000)" _alpha))))))))

(event Custom|Close%20Doors
  (bind (_location _rotation _rotation_control) (|GetRelativeInfo))
  (Utilities|FlowControl|Sequence
    (:then_0
      (Components|MoveComponentTo (Variables|Default|GetDoor%202) "0, 0, 0" "0, 0, 0" false false 0.5 false)
      (bind _alpha (Timeline|TL-Level PlayFromStart)
        (:Update
          (bind _asbp_light (Utilities|Casting|CastToBP-Light (Variables|/Script/Engine.ChildActorComponent|GetChildActor (Variables|Default|GetLight))))
          (Default|UpdateLight _asbp_light (Math|Color|Lerp(LinearColor) "(R=1.000000,G=1.000000,B=1.000000,A=1.000000)" "(R=0.000000,G=0.502886,B=1.000000,A=1.000000)" _alpha)))
        (:Finished
          (Default|SaveRelativeRot/Loc (Variables|Default|GetAs%20GI-Portal) _location _rotation _rotation_control)
          (bind _returnvalue (Utilities|GetDataTableRow "/Game/Blueprints/DT-Levels.DT-Levels" (Variables|Default|GetNext%20Level%20Name))
            (:then
              (Default|SaveGame(LevelProgress) (Variables|Default|GetAs%20GI-Portal) (|ToInt (Variables|Default|GetNext%20Level%20Name)))
              (Game|OpenLevel(byName) (.LevelID (Utilities|Struct|BreakST-Data _returnvalue))))))))
    (:then_1
      (Components|MoveComponentTo (Variables|Default|GetDoor%201) "0, 0, 0" "0, 0, 0" false false 0.5 false))))

(event EventBeginPlay
  (bind _asgi_portal (Utilities|Casting|CastToGI-Portal (Game|GetGameInstance)))
  (Variables|Default|SetAs%20GI-Portal _asgi_portal)
  (if (not (!= "" (Variables|Default|GetNext%20Level%20Name)))
    ;[1 1 1] Spawn
    (CallFunction|OpenDoors true)))

(fn ConstructionScript
  (if (not (!= "" (Variables|Default|GetNext%20Level%20Name)))
    (Components|DestroyComponent (Variables|Default|GetBox-Inside))))