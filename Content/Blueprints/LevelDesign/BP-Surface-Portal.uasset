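; BP-Surface-Portal is a level design Blueprint for a surface portal, defined by a Corner vector and a Type enum.
; Its construction script keeps the Corner's Z from going negative, then derives Type from whether that height is zero or non-zero.
; The event graph holds only disabled default events, so this graph adds no runtime behavior.
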(event EventBeginPlay
  (|CallParentFunction) ; This node is disabled and will not be called.\nDrag off pins to build functionality.
)

(event Collision|EventActorBeginOverlap
  (params (OtherActor :type Actor%20Object%20Reference))
  (|CallParentFunction OtherActor) ; This node is disabled and will not be called.\nDrag off pins to build functionality.
)

(event EventTick
  (params (DeltaSeconds :type Float%20%28single-precision%29))
  (|CallParentFunction DeltaSeconds) ; This node is disabled and will not be called.\nDrag off pins to build functionality.
)

(fn ConstructionScript
  (|CallParentFunction)
  (bind _output_get (Variables|Default|SetCorner (Math|Vector|MakeVector (.x (Variables|Default|GetCorner)) (.y (Variables|Default|GetCorner)) (Math|Float|Clamp(Float) (.z (Variables|Default|GetCorner)) 0.0 (.z (Variables|Default|GetCorner))))))
  (Variables|Default|SetType (select (!= 0.0 (.Z (Math|Vector|BreakVector _output_get))) "NewEnumerator1" "NewEnumerator0")))