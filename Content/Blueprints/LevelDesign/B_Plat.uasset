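; Moving platform for level design that travels along control points in loop-reset or ping-pong fashion.
; Activate configures an InterpToMovement component and starts it after a delay.
; Stop-StartMovement destroys that component and switches to a timeline that lerps the platform point to point, with Speed setting leg duration.
; Toggling it during play sets Cancel, deferring the stop until the index returns to the first point.
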(event Custom|Activate
  (bind _interptomovement (Variables|Default|GetInterpToMovement))
  (Variables|/Script/Engine.InterpToMovementComponent|SetControlPoints _interptomovement (Variables|DefVar|GetControl%20Points))
  (Variables|/Script/Engine.InterpToMovementComponent|SetBehaviourType _interptomovement (Variables|DefVar|GetBehaviour%20Type))
  (Variables|/Script/Engine.InterpToMovementComponent|SetDuration _interptomovement (Variables|DefVar|GetDuration))
  (Class|InterptoMovementComponent|FinaliseControlPoints _interptomovement)
  (Utilities|FlowControl|Delay (Variables|DefVar|GetDelay))
  (Components|Activation|Activate (Variables|Default|GetInterpToMovement) true))

(event Custom|Stop-Start%20Movement
  (params (speed :type Float%20%28double-precision%29))
  (bind (_start _end) (CallFunction|GetLocationLerps))
  (Components|Timeline|SetPlayRate (Variables|Default|GetTL-Move) (/ 1.0 speed))
  (|DestroyInterp)
  (if (not (Audio|Components|Audio|IsPlaying (Variables|Default|GetTL-Move)))
    (Variables|Move|SetCancel false :!label _label)
    (bind _alpha (Timeline|TL-Move Play)
      (:Update
        (Transformation|SetRelativeLocation (Variables|Default|GetPlatform) (Math|Vector|Lerp(Vector) _start _end _alpha) false false))
      (:Finished
        (CallFunction|UpdateCounter)
        (if (and (== (Variables|Move|GetMovement%20Index) 0) (Variables|Move|GetCancel))
          (Components|Timeline|SetNewTime (Variables|Default|GetTL-Move) 0.0)
          (Variables|Move|SetCancel false)
          (else
            (CallFunction|Loop)
            (Components|Timeline|SetNewTime (Variables|Default|GetTL-Move) 0.0)))))
    (elif (Variables|Move|GetCancel)
      (goto _label)
      (else
        (Variables|Move|SetCancel true)
        (Timeline|TL-Move Play)))))

(event Custom|Loop
  (bind (_start _end) (CallFunction|GetLocationLerps))
  (bind _alpha (Timeline|TL-Move Play)
    (:Update
      (Transformation|SetRelativeLocation (Variables|Default|GetPlatform) (Math|Vector|Lerp(Vector) _start _end _alpha) false false))
    (:Finished
      (CallFunction|UpdateCounter)
      (if (and (== (Variables|Move|GetMovement%20Index) 0) (Variables|Move|GetCancel))
        (Components|Timeline|SetNewTime (Variables|Default|GetTL-Move) 0.0)
        (Variables|Move|SetCancel false)
        (else
          (CallFunction|Loop)
          (Components|Timeline|SetNewTime (Variables|Default|GetTL-Move) 0.0))))))

(fn ConstructionScript)

(fn GetLocationLerps
  (return (.positioncontrolpoint (Utilities|Array|Get(acopy) (Variables|DefVar|GetControl%20Points) (Variables|Move|GetMovement%20Index))) (.positioncontrolpoint (Utilities|Array|Get(acopy) (Variables|DefVar|GetControl%20Points) (Math|Integer|SelectInt (Math|Integer|SelectInt (Math|Integer|SelectInt 0 (- (Variables|Move|GetMovement%20Index) 1) (Utilities|Enum|Equal(Enum) (Variables|DefVar|GetBehaviour%20Type) "Loop_Reset")) (+ (Variables|Move|GetMovement%20Index) 1) (> (+ (Variables|Move|GetMovement%20Index) 1) (Utilities|Array|LastIndex (Variables|DefVar|GetControl%20Points)))) (Math|Integer|SelectInt (Math|Integer|SelectInt (Utilities|Array|LastIndex (Variables|DefVar|GetControl%20Points)) 1 (Utilities|Enum|Equal(Enum) (Variables|DefVar|GetBehaviour%20Type) "Loop_Reset")) (- (Variables|Move|GetMovement%20Index) 1) (< (- (Variables|Move|GetMovement%20Index) 1) 0)) (Variables|Move|GetDirection))))))

(fn UpdateCounter
  (if (Variables|Move|GetDirection)
    (if (> (+ (Variables|Move|GetMovement%20Index) 1) (Utilities|Array|LastIndex (Variables|DefVar|GetControl%20Points)))
      (switch Utilities|FlowControl|Switch|SwitchonEInterpToBehaviourType (Variables|DefVar|GetBehaviour%20Type)
        (:Loop_Reset
          (Variables|Move|SetMovement%20Index 0))
        (:PingPong
          (Variables|Move|SetMovement%20Index (- (Utilities|Array|LastIndex (Variables|DefVar|GetControl%20Points)) 1))
          (Variables|Move|SetDirection false)))
      (else
        (bind _result (Math|Integer|IncrementInt (Variables|Move|GetMovement%20Index))
          (:%20%20
            (if (and (== _result (Utilities|Array|LastIndex (Variables|DefVar|GetControl%20Points))) (Utilities|Enum|Equal(Enum) (Variables|DefVar|GetBehaviour%20Type) "Loop_Reset"))
              (Variables|Move|SetMovement%20Index 0))))))
    (elif (< (- (Variables|Move|GetMovement%20Index) 1) 0)
      (switch Utilities|FlowControl|Switch|SwitchonEInterpToBehaviourType (Variables|DefVar|GetBehaviour%20Type)
        (:Loop_Reset
          (Variables|Move|SetMovement%20Index (Utilities|Array|LastIndex (Variables|DefVar|GetControl%20Points))))
        (:PingPong
          (Variables|Move|SetMovement%20Index 1)
          (Variables|Move|SetDirection true)))
      (else
        (Math|Integer|DecrementInt (Variables|Move|GetMovement%20Index))))))