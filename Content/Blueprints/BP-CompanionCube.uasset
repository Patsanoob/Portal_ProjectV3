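; Companion cube actor that gets replaced through its spawner reference when destroyed.
; BeginPlay sizes its collision box and records the spawn transform if unset.
; CubeDestroyed enables mesh physics, plays a Niagara despawn effect, hides the mesh, then asks the spawner for a new cube and destroys itself.
; If destroyed any other way, it requests a respawn only when no other cube shares its ID.
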(event Custom|Cube%20Destroyed
  (bind _spawner_ref (Variables|Default|GetSpawner%20Ref))
  ;[1 1 1] Destroy Cube
  (Variables|Default|SetDestroying true)
  (Physics|SetSimulatePhysics (Variables|Default|GetStaticMeshComponent) true)
  (Niagara|SpawnSystemAttached "/Game/Assets/Particle/NS_CubeDespawn.NS_CubeDespawn" (Variables|Default|GetStaticMeshComponent) "None" "0, 0, 0" (Transformation|GetActorRotation) "KeepRelativeOffset" false)
  (Utilities|FlowControl|Delay 1.0)
  (Development|SetHiddeninGame (Variables|Default|GetStaticMeshComponent) true false)
  (Utilities|FlowControl|Delay 2.5)
  (Utilities|IsValid _spawner_ref
    (:Is%20Valid
      (Default|SpawnCube _spawner_ref))
    (:Is%20Not%20Valid
      _))
  (Actor|DestroyActor))

(event EventBeginPlay
  (Components|Box|SetBoxExtent (Variables|Default|GetBox) "40.000000,40.000000,40.000000" true)
  (if (Utilities|Operators|EqualEqual :A (Variables|Default|GetSpawn%20Loc))
    (Variables|Default|SetSpawn%20Loc (Transformation|GetActorLocation))
    (Variables|Default|SetSpawn%20Rot (Transformation|GetActorRotation))))

(event EventDestroyed
  (CallFunction|DestroyCompanionCube))

(event EventTick
  (params (DeltaSeconds :type Float%20%28single-precision%29))
  (|CallParentFunction DeltaSeconds) ; This node is disabled and will not be called.\nDrag off pins to build functionality.
)

(fn ConstructionScript)

(fn DestroyCompanionCube
  (bind _spawner_ref (Variables|Default|GetSpawner%20Ref))
  (if (not (Variables|Default|GetDestroying))
    (bind _outactors (Actor|GetAllActorsOfClass "BP-CompanionCube_C"))
    (for _array_element _outactors
      (if (!= _array_element self)
        (Utilities|Array|Add (LocalVariables|GetL-Array%20of%20ID) (Variables|/Game/Blueprints/SMA-Carry.SMA-Carry_C|GetID _array_element))))
    (if (not (Utilities|Array|ContainsItem (LocalVariables|GetL-Array%20of%20ID) (Variables|Default|GetID)))
      (Utilities|IsValid _spawner_ref
        (:Is%20Valid
          (Default|SpawnCube _spawner_ref))))))