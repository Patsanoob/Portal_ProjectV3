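; Game instance for a portal game that keeps level progress and carries relative placement data, likely across level transitions.
; On Init it loads the save game from its slot, or creates and saves a new one if none exists.
; Progress is written to disk only when a higher level ID is reached.
; Relative location, rotation and control rotation are stored with a spawn flag and handed back on request.
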(event EventInit
  (bind _returnvalue (SaveGame|DoesSaveGameExist (Variables|Default|GetSaveData)))
  (if _returnvalue
    (bind _returnvalue_2 (SaveGame|LoadGamefromSlot (Variables|Default|GetSaveData)))
    (bind _assg_portal (Utilities|Casting|CastToSG-Portal _returnvalue_2))
    (Variables|Default|SetSaveGame _assg_portal)
    (else
      (bind _returnvalue_3 (SaveGame|CreateSaveGameObject "/Game/Blueprints/SG-Portal.SG-Portal_C"))
      (bind _output_get (Variables|Default|SetSaveGame _returnvalue_3))
      (SaveGame|SaveGametoSlot _output_get (Variables|Default|GetSaveData)))))

(fn SaveRelativeRot/Loc
  (params (Relative%20Location :type Vector) (Relative%20Rotation :type Rotator) (Relative%20Control%20Rotation :type Rotator))
  (Variables|Default|SetRelative%20Location Relative%20Location)
  (Variables|Default|SetRelative%20Rotation Relative%20Rotation)
  (Variables|Default|SetRelative%20Control%20Rotation Relative%20Control%20Rotation)
  (Variables|Default|SetSpawn%20 true))

(fn ShareRelativeRot/Loc
  (return (Variables|Default|GetRelative%20Location) (Variables|Default|GetRelative%20Rotation) (Variables|Default|GetRelative%20Control%20Rotation)))

(fn SaveGame(LevelProgress)
  (params (Level%20ID :type Integer))
  (if (> Level%20ID (Variables|/Game/Blueprints/SG-Portal.SG-Portal_C|GetLevel%20Progress (Variables|Default|GetSaveGame)))
    (Variables|/Game/Blueprints/SG-Portal.SG-Portal_C|SetLevel%20Progress (Variables|Default|GetSaveGame) Level%20ID)
    (SaveGame|SaveGametoSlot (Variables|Default|GetSaveGame) (Variables|Default|GetSaveData))
    (Development|PrintString (Utilities|String|ToString(Integer) (Variables|/Game/Blueprints/SG-Portal.SG-Portal_C|GetLevel%20Progress (Variables|Default|GetSaveGame))))))