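; One of two linked portals (A or B) that shows the view through its partner and manages objects crossing it.
; Each tick it positions the partner's clip-planed scene capture from the player camera and resizes the render target.
; Trigger overlaps relax wall and portal collision and have PC-Portal spawn or destroy player and companion cube clones.
; Energy balls get a replacement spawned at the partner with transformed velocity.
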(event OnComponentBeginOverlap(Trigger-Player)
  (params (OverlappedComponent :type Primitive%20Component%20Object%20Reference) (OtherActor :type Actor%20Object%20Reference) (OtherComp :type Primitive%20Component%20Object%20Reference) (OtherBodyIndex :type Integer) (bFromSweep :type Boolean) (SweepResult :type Hit%20Result%20Structure%20%28by%20ref%29))
  (Overlapping|BeginOverlapEvent OtherActor))

(event OnComponentEndOverlap(Trigger-Player)
  (params (OverlappedComponent :type Primitive%20Component%20Object%20Reference) (OtherActor :type Actor%20Object%20Reference) (OtherComp :type Primitive%20Component%20Object%20Reference) (OtherBodyIndex :type Integer))
  (Overlapping|EndOverlapEvent OtherActor))

(event EventBeginPlay
  (bind _scenecapturecomponent2d (Variables|Default|GetSceneCaptureComponent2D))
  (bind _aspc_portal (Utilities|Casting|CastToPC-Portal (Game|GetPlayerController 0)))
  (Variables|Default|SetAs%20PC-Portal _aspc_portal)
  (CallFunction|DetermineWallsBehindPortal)
  ;[1 1 1] Setup The near clipping planes
  (Variables|/Script/Engine.SceneCaptureComponent2D|SetClipPlaneBase _scenecapturecomponent2d (Transformation|GetWorldLocation (Variables|Default|GetSM-Window)))
  (Variables|/Script/Engine.SceneCaptureComponent2D|SetClipPlaneNormal _scenecapturecomponent2d (Math|Rotator|GetRotationXVector (Transformation|GetActorRotation)))
  (Variables|/Script/Engine.SceneCaptureComponent2D|SetCustomNearClippingPlane _scenecapturecomponent2d 0.0001)
  (|SwaptheCollisionForPlayerifOnFloor)
  (Effects|Components|ParticleSystem|SetColorParameter (Variables|Default|GetNE-Portal) "Portal Color" (Math|Color|SelectColor "(R=25.000000,G=5.000000,B=0.000000,A=1.000000)" "(R=0.000000,G=10.000000,B=20.000000,A=1.000000)" (Variables|Default|GetPortal%20A))))

(event EventTick
  (params (DeltaSeconds :type Float%20%28single-precision%29))
  (Utilities|ValidTickEvent
    (:Is%20Valid
      (CallFunction|UpdatePortalVis))))

(fn ConstructionScript
  (Rendering|Material|SetMaterial (Variables|Default|GetSM-Outline) 0 (select (Variables|Default|GetPortal%20A) "/Game/Assets/Material/MI-PortalA.MI-PortalA" "/Game/Assets/Material/MI-PortalB.MI-PortalB"))
  (Effects|Components|ParticleSystem|SetColorParameter (Variables|Default|GetNE-Portal) "Portal Color" (Math|Color|SelectColor "(R=50.000000,G=10.000000,B=0.000000,A=1.000000)" "(R=0.000000,G=25.000000,B=50.000000,A=1.000000)" (Variables|Default|GetPortal%20A))))

(fn SetupLinkedPortal
  (bind _trigger_player (Variables|Default|GetTrigger-Player))
  (bind _trigger_player_2 (Variables|Default|GetTrigger-Player))
  (bind _trigger_player_3 (Variables|Default|GetTrigger-Player))
  (bind _overlappingactors (Collision|GetOverlappingActors _trigger_player_2 "/Game/Blueprints/Puzzles/BP-EnergyProjectile.BP-EnergyProjectile_C" :!class /Script/Engine.PrimitiveComponent))
  (bind _overlappingactors_2 (Collision|GetOverlappingActors _trigger_player_3 "/Game/FirstPerson/Blueprints/BP_FirstPersonCharacter.BP_FirstPersonCharacter_C" :!class /Script/Engine.PrimitiveComponent))
  (bind _overlappingactors_3 (Collision|GetOverlappingActors _trigger_player "/Game/Blueprints/Puzzles/BP-CompanionCube.BP-CompanionCube_C" :!class /Script/Engine.PrimitiveComponent))
  (bind _output (Utilities|Array|Get(acopy) _overlappingactors))
  (bind _output_2 (Utilities|Array|Get(acopy) _overlappingactors_2))
  (bind _output_3 (Utilities|Array|Get(acopy) _overlappingactors_3))
  (bind _as_pc_portal (Variables|Default|GetAs%20PC-Portal)
    (:then
      (Utilities|IsValid (select (Variables|Default|GetPortal%20A) (Variables|/Game/Blueprints/PC-Portal.PC-Portal_C|GetPortal%20B _as_pc_portal) (Variables|/Game/Blueprints/PC-Portal.PC-Portal_C|GetPortal%20A _as_pc_portal))
        (:Is%20Valid
          (Variables|Default|SetLinked%20Portal (select (Variables|Default|GetPortal%20A) (Variables|/Game/Blueprints/PC-Portal.PC-Portal_C|GetPortal%20B _as_pc_portal) (Variables|/Game/Blueprints/PC-Portal.PC-Portal_C|GetPortal%20A _as_pc_portal)))
          (Variables|/Script/Engine.SceneCaptureComponent2D|SetTextureTarget (Variables|Default|GetSceneCaptureComponent2D) (select (Variables|Default|GetPortal%20A) "/Game/Assets/RenderTargets/RT-PortalA.RT-PortalA" "/Game/Assets/RenderTargets/RT-PortalB.RT-PortalB"))
          (Rendering|Material|SetMaterial (Variables|Default|GetSM-Window) 0 (select (Variables|Default|GetPortal%20A) "/Game/Assets/RenderTargets/MI_PortalRT-B.MI_PortalRT-B" "/Game/Assets/RenderTargets/MI_PortalRT-A.MI_PortalRT-A"))
          (CallFunction|DetermineWallsBehindPortal)
          (Utilities|FlowControl|Sequence
            (:then_0
              ;[1 1 1] Player Overlapping
              (if (> (Utilities|Array|Length _overlappingactors_2) 0)
                (Utilities|IsValid _output_2
                  (:Is%20Valid
                    (Overlapping|BeginOverlapEvent _output_2)))))
            (:then_1
              ;[1 1 1] Cube Overlapping
              (if (> (Utilities|Array|Length _overlappingactors_3) 0)
                (Utilities|IsValid _output_3
                  (:Is%20Valid
                    (Overlapping|BeginOverlapEvent _output_3)))))
            (:then_2
              ;[1 1 1] Energy Ball Overlapping
              (if (> (Utilities|Array|Length _overlappingactors) 0)
                (Utilities|IsValid _output
                  (:Is%20Valid
                    (Overlapping|BeginOverlapEvent _output)))))))))
    (:else)))

(fn FlatWall
  (return (== (.Z (Math|Vector|BreakVector (Transformation|GetActorForwardVector))) 0.0)))

(fn GetEscapeVelocity
  (params (Input%20Velocity :type Vector) (Cube :type Boolean))
  (bind _returnvalue (Transformation|GetActorForwardVector))
  (bind _returnvalue_2 (Transformation|GetActorForwardVector))
  (bind (_x _y) (Math|Vector|BreakVector Input%20Velocity))
  (bind _z (Math|Vector|BreakVector _returnvalue))
  (bind _z_2 (Math|Vector|BreakVector _returnvalue_2))
  (if Cube
    (LocalVariables|SetMin%20Escape%20Velocity (Math|Float|SelectFloat 0.0 (Math|Float|Lerp 0.0 7.5e+02 _z_2) (< _z_2 0.0)))
    (else
      (LocalVariables|SetMin%20Escape%20Velocity (Math|Float|SelectFloat 0.0 (Math|Float|Lerp 0.0 5e+02 _z) (< _z 0.0)))))
  (return (Math|Vector|SelectVector Input%20Velocity (Math|Vector|MakeVector _x _y (LocalVariables|GetMin%20Escape%20Velocity)) (>= (Math|Float|Absolute(Float) (.Z (Math|Vector|BreakVector Input%20Velocity))) (LocalVariables|GetMin%20Escape%20Velocity)))))

(fn BeginOverlapEvent
  (params (Actor%20Overlapping :type Actor%20Object%20Reference))
  (Variables|Default|GetLinked%20Portal
    (:then
      (if (Assist|CheckActorIsinFront Actor%20Overlapping)
        (bind _asbp_first_person_character (Utilities|Casting|CastToBP_FirstPersonCharacter Actor%20Overlapping)
          (:then
            (Utilities|IsValid (Pawn|GetController _asbp_first_person_character)
              (:Is%20Valid
                (LocalVariables|SetPlayer%20Enter _asbp_first_person_character)
                (CallFunction|UpdateWallCollisions "ECR_Ignore")
                (Collision|SetCollisionEnabled (Variables|BP-Portal_C|GetSM-Collision (Variables|Default|GetLinked%20Portal)) "NoCollision")
                (Collision|SetCollisionEnabled (Variables|Default|GetSM-Collision) "QueryAndPhysics")
                (if (.Return%20Value (Default|IsHoldingCube (LocalVariables|GetPlayer%20Enter)))
                  (Default|Spawn-CubeClone (Variables|Default|GetAs%20PC-Portal) self (.Companion%20Cube (Default|IsHoldingCube (LocalVariables|GetPlayer%20Enter))))
                  (Default|SpawnClone (Variables|Default|GetAs%20PC-Portal) self true)
                  (else
                    (Default|SpawnClone (Variables|Default|GetAs%20PC-Portal) self false))))))
          (:CastFailed
            (bind _asbp_companion_cube (Utilities|Casting|CastToBP-CompanionCube Actor%20Overlapping)
              (:then
                (LocalVariables|SetCompanion%20Cube%20Enter _asbp_companion_cube)
                (Default|Spawn-CubeClone (Variables|Default|GetAs%20PC-Portal) self (LocalVariables|GetCompanion%20Cube%20Enter))
                (Default|Swap-Collision (LocalVariables|GetCompanion%20Cube%20Enter) false self)
                ;[1 1 1] Do we need to spawn player clone
                (if (Variables|/Game/Blueprints/Puzzles/BP-CompanionCube.BP-CompanionCube_C|GetHeld (LocalVariables|GetCompanion%20Cube%20Enter))
                  (Default|SpawnClone (Variables|Default|GetAs%20PC-Portal) self true)))
              (:CastFailed
                ;[1 1 1] For Energy Ball
                (Overlapping|EnergyBallOverlap Actor%20Overlapping)))))))
    (:else)))

(fn EndOverlapEvent
  (params (Actor%20Overlapping :type Actor%20Object%20Reference))
  (Variables|Default|GetLinked%20Portal
    (:then
      (if (Assist|CheckActorIsinFront Actor%20Overlapping)
        (Utilities|FlowControl|Sequence
          (:then_0
            (bind _asbp_first_person_character (Utilities|Casting|CastToBP_FirstPersonCharacter Actor%20Overlapping)
              (:then
                (Utilities|IsValid (Pawn|GetController _asbp_first_person_character)
                  (:Is%20Valid
                    (LocalVariables|SetPlayer%20Exit _asbp_first_person_character)
                    (CallFunction|UpdateWallCollisions (Variables|Default|GetLinked%20Portal) "ECR_Block")
                    (if (.Return%20Value (Default|IsHoldingCube (LocalVariables|GetPlayer%20Exit)))
                      (if (not (Collision|IsOverlappingActor (Variables|Default|GetTrigger-Player) (.Companion%20Cube (Default|IsHoldingCube (LocalVariables|GetPlayer%20Exit))) :!class /Script/Engine.PrimitiveComponent)) ; TRUE= Don't Exit\nFALSE= Complete Exit
                        (Default|DestroyClones (Variables|Default|GetAs%20PC-Portal)))
                      (else
                        (Default|DestroyClones (Variables|Default|GetAs%20PC-Portal)))))))
              (:CastFailed
                (bind _asbp_companion_cube (Utilities|Casting|CastToBP-CompanionCube Actor%20Overlapping)
                  (:then
                    (LocalVariables|SetCompanion%20Cube%20Exit _asbp_companion_cube)
                    (|FixCollisionForCube)
                    (if (Variables|/Game/Blueprints/Puzzles/BP-CompanionCube.BP-CompanionCube_C|GetHeld (LocalVariables|GetCompanion%20Cube%20Exit))
                      (if (not (Collision|IsOverlappingActor (Variables|Default|GetTrigger-Player) (Game|GetPlayerCharacter 0) :!class /Script/Engine.PrimitiveComponent)) ; TRUE= Don't Exit\nFALSE= Complete Exit
                        (Default|DestroyClones (Variables|Default|GetAs%20PC-Portal))
                        (Default|DestroyCubeClones (Variables|Default|GetAs%20PC-Portal)))
                      (else
                        (Default|DestroyCubeClone (Variables|Default|GetAs%20PC-Portal) (Variables|Default|GetLinked%20Portal)))))
                  (:CastFailed
                    ;[1 1 1] For Energy Ball
                    (Overlapping|EnergyBallEndOverlap Actor%20Overlapping))))))
          (:then_1
            (if (Collision|IsOverlappingActor Actor%20Overlapping (Variables|Default|GetLinked%20Portal) :!class /Script/Engine.Actor)
              (Overlapping|BeginOverlapEvent (Variables|Default|GetLinked%20Portal) Actor%20Overlapping))))))
    (:else)))

(fn EnergyBallOverlap
  (params (Object :type Actor%20Object%20Reference))
  (Utilities|IsValid (Variables|Default|GetLinked%20Portal)
    (:Is%20Valid
      (bind _asbp_energy_projectile (Utilities|Casting|CastToBP-EnergyProjectile Object))
      (bind _output_get (LocalVariables|SetTemp-ProjectileRef _asbp_energy_projectile))
      (LocalVariables|SetVelocity%20Of%20Object (Transformation|GetVelocity _output_get))
      (bind (_outhit _returnvalue) (Collision|LineTraceForObjects (Transformation|GetActorLocation (LocalVariables|GetTemp-ProjectileRef)) (+ (Transformation|GetActorLocation (LocalVariables|GetTemp-ProjectileRef)) (LocalVariables|GetVelocity%20Of%20Object)) (Utilities|Array|MakeArray "ObjectTypeQuery10") true (Utilities|Array|MakeArray (Variables|Default|GetLinked%20Portal)) "None" false "(R=1.000000,G=0.000000,B=0.000000,A=1.000000)" "(R=0.000000,G=1.000000,B=0.000000,A=1.000000)" 0.3))
      (if _returnvalue
        (if (== (.HitComponent (Collision|BreakHitResult _outhit)) (Variables|Default|GetSM-Window))
          (if (<= (Math|Vector|DotProduct (Math|Vector|Normalize (- (+ (LocalVariables|GetVelocity%20Of%20Object) (Transformation|GetActorLocation (LocalVariables|GetTemp-ProjectileRef))) (Transformation|GetActorLocation))) (Transformation|GetActorForwardVector)) 0.0)
            (Collision|SetCollisionResponsetoChannel (Variables|/Game/Blueprints/Puzzles/BP-EnergyProjectile.BP-EnergyProjectile_C|GetCollisionComponent (LocalVariables|GetTemp-ProjectileRef)) "ECC_GameTraceChannel4" "ECR_Overlap")
            (Collision|SetCollisionResponsetoChannel (Variables|/Game/Blueprints/Puzzles/BP-EnergyProjectile.BP-EnergyProjectile_C|GetCollisionComponent (LocalVariables|GetTemp-ProjectileRef)) "ECC_GameTraceChannel3" "ECR_Overlap")
            (Collision|SetCollisionResponsetoChannel (Variables|Default|GetSM-Window) "ECC_GameTraceChannel1" "ECR_Overlap")
            (Collision|SetCollisionObjectType (Variables|Default|GetSM-Collision) "ECC_WorldStatic")
            (bind _returnvalue_2 (Game|SpawnActorfromClass "/Game/Blueprints/Puzzles/BP-EnergyProjectile.BP-EnergyProjectile_C" (Math|Transform|MakeTransform (Math|Transform|TransformLocation (Transformation|GetWorldTransform (Variables|BP-Portal_C|GetOpposite%20Scene (Variables|Default|GetLinked%20Portal))) (Math|Transform|InverseTransformLocation (Transformation|GetActorTransform) (Transformation|GetActorLocation (LocalVariables|GetTemp-ProjectileRef))))) "Undefined" 0 (Variables|/Game/Blueprints/Puzzles/BP-EnergyProjectile.BP-EnergyProjectile_C|GetSpawnerRef (LocalVariables|GetTemp-ProjectileRef)) 0))
            (bind _output_get_2 (LocalVariables|SetClone-ProjectileRef _returnvalue_2))
            (Niagara|ResetSystem (Variables|/Game/Blueprints/Puzzles/BP-EnergyProjectile.BP-EnergyProjectile_C|GetNiagara (LocalVariables|GetTemp-ProjectileRef)))
            (Variables|/Script/Engine.MovementComponent|SetVelocity (Variables|/Game/Blueprints/Puzzles/BP-EnergyProjectile.BP-EnergyProjectile_C|GetProjectileMovement _output_get_2) (Math|Transform|TransformDirection (Transformation|GetWorldTransform (Variables|BP-Portal_C|GetOpposite%20Scene (Variables|Default|GetLinked%20Portal))) (Math|Transform|InverseTransformDirection (Transformation|GetActorTransform) (LocalVariables|GetVelocity%20Of%20Object))))
            (Variables|/Game/Blueprints/Puzzles/BP-ProjectileSpawner.BP-ProjectileSpawner_C|SetEnergyBall-Ref (Variables|/Game/Blueprints/Puzzles/BP-EnergyProjectile.BP-EnergyProjectile_C|GetSpawnerRef (LocalVariables|GetTemp-ProjectileRef)) (LocalVariables|GetClone-ProjectileRef))
            (Variables|/Game/Blueprints/Puzzles/BP-EnergyProjectile.BP-EnergyProjectile_C|SetBounce%20Count (LocalVariables|GetClone-ProjectileRef) (Variables|/Game/Blueprints/Puzzles/BP-EnergyProjectile.BP-EnergyProjectile_C|GetBounce%20Count (LocalVariables|GetTemp-ProjectileRef)))
            (Collision|SetCollisionResponsetoChannel (Variables|/Game/Blueprints/Puzzles/BP-EnergyProjectile.BP-EnergyProjectile_C|GetCollisionComponent (LocalVariables|GetClone-ProjectileRef)) "ECC_GameTraceChannel4" "ECR_Overlap")
            (Collision|SetCollisionResponsetoChannel (Variables|/Game/Blueprints/Puzzles/BP-EnergyProjectile.BP-EnergyProjectile_C|GetCollisionComponent (LocalVariables|GetClone-ProjectileRef)) "ECC_GameTraceChannel3" "ECR_Overlap")
            (Variables|Default|SetOld%20Overlapping%20Projectile (LocalVariables|GetTemp-ProjectileRef))))))))

(fn EnergyBallEndOverlap
  (params (Object :type Actor%20Object%20Reference))
  (bind _asbp_energy_projectile (Utilities|Casting|CastToBP-EnergyProjectile Object))
  (if (not (== (Variables|Default|GetOld%20Overlapping%20Projectile) _asbp_energy_projectile))
    (LocalVariables|SetEnergyBall_Ref _asbp_energy_projectile)
    ;[1 1 1] Fix Collisions
    (Collision|SetCollisionResponsetoChannel (Variables|BP-Portal_C|GetSM-Window (Variables|Default|GetLinked%20Portal)) "ECC_GameTraceChannel1" "ECR_Block")
    (Collision|SetCollisionResponsetoChannel (Variables|/Game/Blueprints/Puzzles/BP-EnergyProjectile.BP-EnergyProjectile_C|GetCollisionComponent (LocalVariables|GetEnergyBall_Ref)) "ECC_GameTraceChannel4" "ECR_Block")
    (Collision|SetCollisionResponsetoChannel (Variables|/Game/Blueprints/Puzzles/BP-EnergyProjectile.BP-EnergyProjectile_C|GetCollisionComponent (LocalVariables|GetEnergyBall_Ref)) "ECC_GameTraceChannel3" "ECR_Block")
    (Collision|SetCollisionObjectType (Variables|Default|GetSM-Collision) "ECC_GameTraceChannel4")
    (Utilities|IsValid (Variables|Default|GetOld%20Overlapping%20Projectile)
      (:Is%20Valid
        (Actor|DestroyActor (Variables|Default|GetOld%20Overlapping%20Projectile))
        (Variables|Default|SetOld%20Overlapping%20Projectile 0)))))

(fn IgnoreCubeCollisiononWall
  (for _array_element (Variables|Default|GetArray%20Of%20Walls%20To%20Hide)
    (Collision|SetCollisionResponsetoChannel (Variables|/Game/Blueprints/LevelDesign/BP_SurfaceV2.BP_SurfaceV2_C|GetSM_Surface _array_element) "ECC_GameTraceChannel8" "ECR_Ignore")))

(fn FixCubeCollisiononWall
  (for _array_element (Variables|Default|GetArray%20Of%20Walls%20To%20Hide)
    (Collision|SetCollisionResponsetoChannel (Variables|/Game/Blueprints/LevelDesign/BP_SurfaceV2.BP_SurfaceV2_C|GetSM_Surface _array_element) "ECC_GameTraceChannel8" "ECR_Block")))

(fn CheckActorIsinFront
  (params (ActorIn :type Actor%20Object%20Reference))
  (return (> (Math|Vector|DotProduct (Math|Vector|Normalize (- (Transformation|GetActorLocation ActorIn) (Transformation|GetActorLocation))) (Transformation|GetActorForwardVector)) 0.0)))

(fn UpdateWallCollisions
  (params (Response :type ECollisionResponse%20Enum :default "ECR_Ignore"))
  (LocalVariables|SetNew%20Response Response)
  (for _array_element (Variables|Default|GetArray%20Of%20Walls%20To%20Hide)
    (Collision|SetCollisionResponsetoChannel (Variables|/Game/Blueprints/LevelDesign/BP_SurfaceV2.BP_SurfaceV2_C|GetSM_Surface _array_element) "ECC_Pawn" (LocalVariables|GetNew%20Response)))
  (return))

(fn GetWallHit
  (return (Utilities|Array|Get(acopy) (Variables|Default|GetArray%20Of%20Walls%20To%20Hide))))

(fn DetermineWallsBehindPortal
  (bind _returnvalue (Transformation|GetActorLocation))
  (bind _outhits (Class|KismetSystemLibrary|BoxTraceMultiforObjects (- _returnvalue "") (- _returnvalue "-1.000000,0.000000,0.000000") "1.000000,100.000000,140.000000" (Transformation|GetActorRotation) (Utilities|Array|MakeArray "ObjectTypeQuery9") false 0 "None" true))
  (for _array_element _outhits
    (bind _asbp_surface__portal (Utilities|Casting|CastToBP_Surface-Portal (.HitActor (Collision|BreakHitResult _array_element))))
    (if (Utilities|Operators|EqualEqual (Math|Vector|GetUpVector (Variables|/Game/Blueprints/LevelDesign/BP_SurfaceV2.BP_SurfaceV2_C|GetSM_Surface _asbp_surface__portal)) (Transformation|GetActorForwardVector) 0.01)
      (Utilities|Array|AddUnique (Variables|Default|GetArray%20Of%20Walls%20To%20Hide) _asbp_surface__portal)
      (Utilities|Array|Add (Variables|Default|GetArray%20Of%20Actors%20To%20Hide) _asbp_surface__portal))))

(fn IsOverlappingInvalidActor
  (for _array_element (Class|PrimitiveComponent|GetOverlappingComponents (Variables|Default|GetSpawn%20Detection))
    (if (not (or (Utilities|Enum|Equal(Enum) (Collision|GetCollisionObjectType _array_element) "ECC_GameTraceChannel7") (Utilities|Enum|Equal(Enum) (Collision|GetCollisionObjectType _array_element) "ECC_GameTraceChannel2")))
      (if (Utilities|Operators|NotEqual(!=) (Math|Vector|GetUpVector _array_element) (Transformation|GetActorForwardVector) 0.01)
        (return true))
      (else
        (return true))))
  (return false))

(fn UpdatePortalVis
  (bind (_returnvalue_x _returnvalue_y) (|GetRenderTargetSize))
  (Class|PortalLibrary|ResizeRenderTarget (Variables|/Script/Engine.SceneCaptureComponent2D|GetTextureTarget (Variables|Default|GetSceneCaptureComponent2D)) _returnvalue_x _returnvalue_y)
  ;[1 1 1] Modify location of scene capture of the other portal
  (bind _as_pc_portal (Variables|Default|GetAs%20PC-Portal)
    (:then
      (Transformation|SetRelativeLocationAndRotation (Variables|BP-Portal_C|GetSceneCaptureComponent2D (Variables|Default|GetLinked%20Portal)) (.location (Class|KismetMathLibrary|ConvertTransformtoRelative (Transformation|GetWorldTransform (Variables|Default|GetOpposite%20Scene)) (Transformation|GetWorldTransform (Variables|/Game/FirstPerson/Blueprints/BP_FirstPersonCharacter.BP_FirstPersonCharacter_C|GetFirstPersonCamera (Variables|/Game/Blueprints/PC-Portal.PC-Portal_C|GetAs%20BP%20FPC _as_pc_portal))))) (.rotation (Class|KismetMathLibrary|ConvertTransformtoRelative (Transformation|GetWorldTransform (Variables|Default|GetOpposite%20Scene)) (Transformation|GetWorldTransform (Variables|/Game/FirstPerson/Blueprints/BP_FirstPersonCharacter.BP_FirstPersonCharacter_C|GetFirstPersonCamera (Variables|/Game/Blueprints/PC-Portal.PC-Portal_C|GetAs%20BP%20FPC _as_pc_portal))))) false false))
    (:else)))